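; Player component that turns first-person interactions with objects and NPCs into actions for an LLM-driven simulation.
; Left click picks up or drops objects; right click pairs the held object or hand with the traced target as JSON instigator and receiver.
; These feed StateManager's managers and action list, or open HUD action-type selection when toggled.
; A timer trace drives HUD info and custom-depth highlighting; keys focus text input and print actions.
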(event Custom|DetectItemInFront
  (CallFunction|DetectObjects))

(event EventBeginPlay
  (bind _self self)
  (Utilities|FlowControl|Sequence
    (:then_0
      (Variables|Default|SetObjectJSON (Utilities|Struct|MakeJsonObjectWrapper))
      (Variables|Default|SetIgnoreActors (Actor|GetAllChildActors (Components|GetOwner self) true))
      (bind _outactors (Actor|GetAllActorsOfClass "/Game/LLMComunication/StateManager.StateManager_C"))
      (for _array_element _outactors
        (Variables|Default|SetStateManager _array_element)
        (Utilities|Array|Add (Variables|/Script/Engine.Actor|GetTags (Components|GetOwner _self)) (Utilities|String|StringToName "Player"))
        (bind _returnvalue (UserInterface|CreateWidget "/Game/LLMComunication/WindowInput_Final.WindowInput_Final_C"))
        (Variables|Default|SetInputWindowFinal _returnvalue)
        (Variables|/Game/LLMComunication/WindowInput_Final.WindowInput_Final_C|SetWindowPlayer (Variables|Default|GetInputWindowFinal) _self)
        (UserInterface|Viewport|AddtoViewport _returnvalue 0)
        (Input|SetInputModeGameOnly (Game|GetPlayerController 0) false)
        (bind _returnvalue_2 (UserInterface|CreateWidget "/Game/LLMComunication/LlmHUD.LlmHUD_C"))
        (bind _output_get (Variables|Default|SetLLM_HUD _returnvalue_2))
        (UserInterface|Viewport|AddtoViewport _output_get 0)
        (Default|SetLlmHud _output_get false)))
    (:then_1
      (bind _output_get_2 (Variables|Default|SetOwnerCamera (Actor|GetComponentbyClass (Components|GetOwner) "/Script/Engine.CameraComponent")))
      (if (and (Utilities|IsValid _output_get_2) (Utilities|IsValid (Variables|Default|GetLLM_HUD)))
        (Utilities|Time|SetTimerbyEvent (delegate Custom|DetectItemInFront) 0.1 true)))))

(event Input|KeyboardEvents|M
  (params (Key :type Key%20Structure :default "None"))
  (:Released
    (bind _output_get (Variables|Default|SetSelectActionType (not (Variables|Default|GetSelectActionType))))
    (Default|ChangeInteractionMode (Variables|Default|GetLLM_HUD) _output_get)))

(event Input|MouseEvents|RightMouseButton
  (params (Key :type Key%20Structure :default "None"))
  (bind _self self)
  (bind _statemanager (Variables|Default|GetStateManager))
  (bind _objectactor (Variables|Default|GetObjectActor))
  (bind _returnvalue (Components|GetOwner _self))
  (bind _returnvalue_2 (Actor|GetComponentbyClass _objectactor "/Game/LLMComunication/BP_ObjectInfo.BP_ObjectInfo_C"))
  (bind _globalmanager (Variables|/Game/LLMComunication/StateManager.StateManager_C|GetGlobalManager _statemanager))
  (bind _prompmanager (Variables|/Game/LLMComunication/StateManager.StateManager_C|GetPrompManager _statemanager))
  (bind _returnvalue_3 (Actor|GetComponentbyClass _returnvalue "/Script/Engine.CameraComponent"))
  (bind _originalscene (Variables|/Game/LLMComunication/BP_ObjectInfo.BP_ObjectInfo_C|GetOriginalScene _returnvalue_2))
  (bind _returnvalue_4 (Transformation|GetWorldLocation _returnvalue_3))
  (:Released
    (bind _outhit (Collision|LineTraceByChannel _returnvalue_4 (+ _returnvalue_4 (* (Math|Vector|GetForwardVector _returnvalue_3) (Variables|Default|GetRaycastDistance))) "TraceTypeQuery1" false (Variables|Default|GetIgnoreActors) "ForDuration" true "(R=1.000000,G=0.000000,B=0.000000,A=1.000000)" "(R=0.000000,G=1.000000,B=0.000000,A=1.000000)" 2.0))
    (Utilities|IsValid (.HitActor (Collision|BreakHitResult _outhit))
      (:Is%20Valid
        (Utilities|IsValid (Actor|GetComponentbyClass (.HitActor (Collision|BreakHitResult _outhit)) "/Game/LLMComunication/BP_ObjectInfo.BP_ObjectInfo_C")
          (:Is%20Valid
            (if (not (Variables|/Game/LLMComunication/BP_ObjectInfo.BP_ObjectInfo_C|GetProcessing (Actor|GetComponentbyClass (.HitActor (Collision|BreakHitResult _outhit)) "/Game/LLMComunication/BP_ObjectInfo.BP_ObjectInfo_C")))
              (if (Utilities|IsValid (Variables|Default|GetObjectActor)) :!label _label
                (bind _json_string (Default|CreateObjectInfo _returnvalue_2))
                (Variables|Default|SetInstigator _json_string)
                (if (Utilities|IsValid (Actor|GetComponentbyClass (.HitActor (Collision|BreakHitResult _outhit)) "/Game/LLMComunication/BP_NPCInfo.BP_NPCInfo_C"))
                  (bind _asinteractive_obj (Utilities|Casting|CastToInteractiveObj _objectactor))
                  (Default|IsProcessing _asinteractive_obj true)
                  (Default|SetInstigator (Variables|/Game/LLMComunication/StateManager.StateManager_C|GetGlobalManager (Variables|Default|GetStateManager)) _asinteractive_obj)
                  (if _originalscene
                    (Variables|/Game/LLMComunication/PrompManager.PrompManager_C|SetInstigatorInteractiveObj _prompmanager _asinteractive_obj))
                  (bind _json_string_2 (CallFunction|CreateNPCInfo (.HitActor (Collision|BreakHitResult _outhit)) :!label _label_2))
                  (Variables|Default|SetReceiver _json_string_2)
                  (CallFunction|DetachObject)
                  (if (Variables|Default|GetSelectActionType)
                    (Default|SetActionType (Variables|Default|GetLLM_HUD) true)
                    (else
                      (CallFunction|AddAction "interact" true)))
                  (else
                    (bind _asinteractive_obj_2 (Utilities|Casting|CastToInteractiveObj _objectactor))
                    (Default|IsProcessing _asinteractive_obj_2 true)
                    (Default|SetInstigator _globalmanager _asinteractive_obj_2)
                    (if _originalscene
                      (Variables|/Game/LLMComunication/PrompManager.PrompManager_C|SetInstigatorInteractiveObj _prompmanager _asinteractive_obj_2))
                    (bind _json_string_3 (Default|CreateObjectInfo (Actor|GetComponentbyClass (.HitActor (Collision|BreakHitResult _outhit)) "/Game/LLMComunication/BP_ObjectInfo.BP_ObjectInfo_C") :!label _label_3))
                    (Variables|Default|SetReceiver _json_string_3)
                    (Default|IsProcessing (Variables|/Game/LLMComunication/BP_ObjectInfo.BP_ObjectInfo_C|GetInteractiveObj (Actor|GetComponentbyClass (.HitActor (Collision|BreakHitResult _outhit)) "/Game/LLMComunication/BP_ObjectInfo.BP_ObjectInfo_C")) true)
                    (Default|SetReceiver _globalmanager (Variables|/Game/LLMComunication/BP_ObjectInfo.BP_ObjectInfo_C|GetInteractiveObj (Actor|GetComponentbyClass (.HitActor (Collision|BreakHitResult _outhit)) "/Game/LLMComunication/BP_ObjectInfo.BP_ObjectInfo_C")))
                    (if (Variables|/Game/LLMComunication/BP_ObjectInfo.BP_ObjectInfo_C|GetOriginalScene (Actor|GetComponentbyClass (.HitActor (Collision|BreakHitResult _outhit)) "/Game/LLMComunication/BP_ObjectInfo.BP_ObjectInfo_C"))
                      (Variables|/Game/LLMComunication/PrompManager.PrompManager_C|SetReciverInteractiveObj _prompmanager (Variables|/Game/LLMComunication/BP_ObjectInfo.BP_ObjectInfo_C|GetInteractiveObj (Actor|GetComponentbyClass (.HitActor (Collision|BreakHitResult _outhit)) "/Game/LLMComunication/BP_ObjectInfo.BP_ObjectInfo_C"))))
                    (CallFunction|DetachObject)
                    (if (Variables|Default|GetSelectActionType)
                      (Default|SetActionType (Variables|Default|GetLLM_HUD) false)
                      (else
                        (CallFunction|AddAction "interact" false)))))
                (else
                  (Variables|Default|SetInstigator "{\"name\":\"Player (interacting with its hand )\"}")
                  (Variables|/Game/LLMComunication/PrompManager.PrompManager_C|SetPlayerInstigator (Variables|/Game/LLMComunication/StateManager.StateManager_C|GetPrompManager (Variables|Default|GetStateManager)) true)
                  (if (Utilities|IsValid (Actor|GetComponentbyClass (.HitActor (Collision|BreakHitResult _outhit)) "/Game/LLMComunication/BP_NPCInfo.BP_NPCInfo_C"))
                    (goto _label_2)
                    (else
                      (goto _label_3)))))
              (else
                (Utilities|IsValid (Actor|GetComponentbyClass (.HitActor (Collision|BreakHitResult _outhit)) "/Game/LLMComunication/BP_NPCInfo.BP_NPCInfo_C") :!label _label_4
                  (:Is%20Valid
                    (if (not (Variables|/Game/LLMComunication/BP_NPCInfo.BP_NPCInfo_C|GetDead (Actor|GetComponentbyClass (.HitActor (Collision|BreakHitResult _outhit)) "/Game/LLMComunication/BP_NPCInfo.BP_NPCInfo_C")))
                      (if (not (Variables|/Game/LLMComunication/BP_NPCInfo.BP_NPCInfo_C|GetIsProcessing (Actor|GetComponentbyClass (.HitActor (Collision|BreakHitResult _outhit)) "/Game/LLMComunication/BP_NPCInfo.BP_NPCInfo_C")))
                        (goto _label))))))))
          (:Is%20Not%20Valid
            (goto _label_4)))))))

(event Input|KeyboardEvents|R
  (params (Key :type Key%20Structure :default "None"))
  (:Released
    (bind _actionsjson (Default|GetActions (Variables|Default|GetStateManager)))
    (Development|PrintString _actionsjson true true "(R=1.000000,G=0.000000,B=0.022203,A=1.000000)")))

(event Input|MouseEvents|LeftMouseButton
  (params (Key :type Key%20Structure :default "None"))
  (bind _self self)
  (bind _objectplacement (Variables|Default|GetObjectPlacement))
  (bind _returnvalue (Components|GetOwner _self))
  (bind (_x _y _z) (Class|KismetMathLibrary|BreakVector3f _objectplacement))
  (bind _returnvalue_2 (Actor|GetComponentbyClass _returnvalue "/Script/Engine.CameraComponent"))
  (bind _returnvalue_3 (Transformation|GetWorldLocation _returnvalue_2))
  (bind _returnvalue_4 (Math|Vector|GetForwardVector _returnvalue_2))
  (:Released
    (if (Utilities|IsValid (Variables|Default|GetObjectActor))
      (CallFunction|DetachObject)
      (else
        (bind (_outhit _returnvalue_5) (Collision|LineTraceByChannel _returnvalue_3 (+ _returnvalue_3 (* _returnvalue_4 (Variables|Default|GetRaycastDistance))) "TraceTypeQuery1" false (Variables|Default|GetIgnoreActors) "ForDuration" true "(R=0.783381,G=0.000000,B=1.000000,A=1.000000)" "(R=0.000000,G=1.000000,B=0.000000,A=1.000000)" 2.0))
        (if _returnvalue_5
          (Utilities|IsValid (.HitActor (Collision|BreakHitResult _outhit))
            (:Is%20Valid
              (Utilities|IsValid (Actor|GetComponentbyClass (.HitActor (Collision|BreakHitResult _outhit)) "/Game/LLMComunication/BP_ObjectInfo.BP_ObjectInfo_C")
                (:Is%20Valid
                  (if (not (Variables|/Game/LLMComunication/BP_ObjectInfo.BP_ObjectInfo_C|GetProcessing (Actor|GetComponentbyClass (.HitActor (Collision|BreakHitResult _outhit)) "/Game/LLMComunication/BP_ObjectInfo.BP_ObjectInfo_C")))
                    (bind _isinteractuable (Default|IsInteractuable (Actor|GetComponentbyClass (.HitActor (Collision|BreakHitResult _outhit)) "/Game/LLMComunication/BP_ObjectInfo.BP_ObjectInfo_C")))
                    (if _isinteractuable
                      (bind _output_get (Variables|Default|SetObjectActor (.HitActor (Collision|BreakHitResult _outhit))))
                      (Transformation|SetActorLocation _output_get (+ _returnvalue_3 (+ (* _returnvalue_4 _z) (* (Math|Vector|GetRightVector _returnvalue_2) _x) (* (Math|Vector|GetUpVector _returnvalue_2) _y))) false true)
                      (Transformation|AttachActorToActor _output_get (Components|GetOwner self) "None" "KeepWorld" "KeepRelative" "KeepRelative" true)
                      (Utilities|Array|Add (Variables|Default|GetIgnoreActors) _output_get))))))))))))

(event Input|KeyboardEvents|T
  (params (Key :type Key%20Structure :default "None"))
  (bind _inputwindowfinal (Variables|Default|GetInputWindowFinal))
  (:Released
    (Input|SetInputModeUIOnly (Game|GetPlayerController 0) _inputwindowfinal "DoNotLock" false)
    (Widget|SetFocus _inputwindowfinal)))

(fn ChangeObjectState
  (bind _interactiveobj (Variables|Default|GetInteractiveObj))
  (bind _asdoor_state_machine (Utilities|Casting|CastToDoorStateMachine (Variables|/Game/LLMComunication/InteractiveObj.InteractiveObj_C|GetStateMachine _interactiveobj)))
  (if (Utilities|Enum|Equal(Enum) (Variables|/Game/LLMComunication/Pruebas/DoorStateMachine.DoorStateMachine_C|GetCurrState _asdoor_state_machine) "Open")
    (Default|ChangeState _interactiveobj "Close")
    (else
      (Default|ChangeState _interactiveobj "Open")))
  (Development|PrintString "INTERACTUANDO" true true "(R=0.000000,G=0.660000,B=1.000000,A=1.000000)" 5.0))

(fn CreateNPCInfo
  (params (Object :type Object%20Object%20Reference))
  (bind _statemanager (Variables|Default|GetStateManager))
  (bind _assimulation_npc (Utilities|Casting|CastToSimulationNPC Object))
  (Variables|/Game/LLMComunication/PrompManager.PrompManager_C|SetNPC (Variables|/Game/LLMComunication/StateManager.StateManager_C|GetPrompManager _statemanager) _assimulation_npc)
  (Default|SetNPCs (Variables|/Game/LLMComunication/StateManager.StateManager_C|GetGlobalManager _statemanager) (Utilities|Array|MakeArray _assimulation_npc))
  (Default|Think _assimulation_npc true)
  (bind _outjsonobject (Class|JsonBlueprintFunctionLibrary|FromString "{}"))
  (bind _output_get (Variables|Default|SetObjectJSON _outjsonobject))
  (|SetJsonField _output_get "Identity" (Variables|/Game/LLMComunication/SimulationNPC.SimulationNPC_C|GetNPCIdentity _assimulation_npc))
  (|SetJsonField _output_get "context" (Variables|/Game/LLMComunication/SimulationNPC.SimulationNPC_C|GetContext _assimulation_npc))
  (bind _outjsonstring (Class|JsonBlueprintFunctionLibrary|ToString _output_get))
  (return _outjsonstring))

(fn DetectObjects
  (bind _ownercamera (Variables|Default|GetOwnerCamera))
  (bind _returnvalue (Transformation|GetWorldLocation _ownercamera))
  (bind (_outhit _returnvalue_2) (Collision|LineTraceByChannel _returnvalue (+ _returnvalue (* (Math|Vector|GetForwardVector _ownercamera) (Variables|Default|GetRaycastDistance))) "TraceTypeQuery1" false (Utilities|Array|MakeArray (Components|GetOwner)) "None"))
  (if _returnvalue_2
    (LocalVariables|SetHitActor (.HitActor (Collision|BreakHitResult _outhit)))
    (LocalVariables|SetSameActorDetected (== (Variables|Default|GetLastDetectedActor) (LocalVariables|GetHitActor)))
    (Utilities|IsValid (Actor|GetComponentbyClass (LocalVariables|GetHitActor) "/Game/LLMComunication/BP_ObjectInfo.BP_ObjectInfo_C")
      (:Is%20Valid
        (Default|DetectedNewObject (Variables|Default|GetLLM_HUD) true (Variables|/Game/LLMComunication/BP_ObjectInfo.BP_ObjectInfo_C|GetProcessing (Actor|GetComponentbyClass (LocalVariables|GetHitActor) "/Game/LLMComunication/BP_ObjectInfo.BP_ObjectInfo_C")) (Variables|/Game/LLMComunication/BP_ObjectInfo.BP_ObjectInfo_C|GetName (Actor|GetComponentbyClass (LocalVariables|GetHitActor) "/Game/LLMComunication/BP_ObjectInfo.BP_ObjectInfo_C")) (Variables|/Game/LLMComunication/BP_ObjectInfo.BP_ObjectInfo_C|GetDescription (Actor|GetComponentbyClass (LocalVariables|GetHitActor) "/Game/LLMComunication/BP_ObjectInfo.BP_ObjectInfo_C")))
        (if (not (LocalVariables|GetSameActorDetected)) :!label _label
          (Utilities|IsValid (Variables|Default|GetLastDetectedStaticMesh)
            (:Is%20Valid
              (Rendering|SetRenderCustomDepth (Variables|Default|GetLastDetectedStaticMesh) false))
            (:Is%20Not%20Valid
              _))
          (Variables|Default|SetLastDetectedStaticMesh (Actor|GetComponentbyClass (LocalVariables|GetHitActor) "/Script/Engine.MeshComponent"))
          (Rendering|SetRenderCustomDepth (Actor|GetComponentbyClass (LocalVariables|GetHitActor) "/Script/Engine.MeshComponent") true)
          (Variables|Default|SetLastDetectedActor (LocalVariables|GetHitActor))))
      (:Is%20Not%20Valid
        (Utilities|IsValid (Actor|GetComponentbyClass (LocalVariables|GetHitActor) "/Game/LLMComunication/BP_NPCInfo.BP_NPCInfo_C")
          (:Is%20Valid
            (goto _label))
          (:Is%20Not%20Valid
            (Default|DetectedNewObject (Variables|Default|GetLLM_HUD) false false :!label _label_2)
            (Variables|Default|SetLastDetectedActor 0)
            (Utilities|IsValid (Variables|Default|GetLastDetectedStaticMesh)
              (:Is%20Valid
                (Rendering|SetRenderCustomDepth (Variables|Default|GetLastDetectedStaticMesh) false)
                (Variables|Default|SetLastDetectedStaticMesh 0)))))))
    (else
      (goto _label_2))))

(fn DetachObject
  (bind _ignoreactors (Variables|Default|GetIgnoreActors))
  (Utilities|IsValid (Variables|Default|GetObjectActor)
    (:Is%20Valid
      (Transformation|DetachFromActor (Variables|Default|GetObjectActor) "KeepWorld" "KeepWorld" "KeepWorld")
      (Utilities|IsValid (Actor|GetComponentbyClass (Variables|Default|GetObjectActor) "/Script/Engine.StaticMeshComponent")
        (:Is%20Valid
          (Physics|SetSimulatePhysics (Actor|GetComponentbyClass (Variables|Default|GetObjectActor) "/Script/Engine.StaticMeshComponent") true))
        (:Is%20Not%20Valid
          _))
      (Variables|Default|SetObjectActor 0)
      (Utilities|Array|RemoveIndex _ignoreactors (- (Utilities|Array|Length _ignoreactors) 1)))))

(fn AddAction
  (params (Type :type String) (NPC-Object :type Boolean))
  (Default|AddAction (Variables|Default|GetStateManager) (Variables|Default|GetInstigator) (Variables|Default|GetReceiver) Type NPC-Object))