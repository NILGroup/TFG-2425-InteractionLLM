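; BP_NPCInfo builds a JSON description of the SimulationNPC that owns it, as part of the LLM communication code.
; CreateNPCInfo first registers the owner with its StateManager's prompt manager and sets it as the sole entry in the GlobalManager's NPC list.
; It then calls Think on the NPC and returns its identity and context serialized as a JSON string.
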(event EventBeginPlay)

(event EventTick
  (params (DeltaSeconds :type Float%20%28single-precision%29)))

(fn CreateNPCInfo
  (bind _assimulation_npc (Utilities|Casting|CastToSimulationNPC (Components|GetOwner)))
  (Variables|/Game/LLMComunication/PrompManager.PrompManager_C|SetNPC (Variables|/Game/LLMComunication/StateManager.StateManager_C|GetPrompManager (Variables|/Game/LLMComunication/SimulationNPC.SimulationNPC_C|GetStateManager _assimulation_npc)) _assimulation_npc)
  (Default|SetNPCs (Variables|/Game/LLMComunication/StateManager.StateManager_C|GetGlobalManager (Variables|/Game/LLMComunication/SimulationNPC.SimulationNPC_C|GetStateManager _assimulation_npc)) (Utilities|Array|MakeArray _assimulation_npc))
  (Default|Think _assimulation_npc true)
  (bind _outjsonobject (Class|JsonBlueprintFunctionLibrary|FromString "{}"))
  (bind _output_get (LocalVariables|SetObjectJSON _outjsonobject))
  (|SetJsonField _output_get "Identity" (Variables|/Game/LLMComunication/SimulationNPC.SimulationNPC_C|GetNPCIdentity _assimulation_npc))
  (|SetJsonField _output_get "context" (Variables|/Game/LLMComunication/SimulationNPC.SimulationNPC_C|GetContext _assimulation_npc))
  (bind _outjsonstring (Class|JsonBlueprintFunctionLibrary|ToString _output_get))
  (return _outjsonstring))