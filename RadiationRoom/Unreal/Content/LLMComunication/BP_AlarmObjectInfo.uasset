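; BP_AlarmObjectInfo is the alarm's interactable object info Blueprint, turning an alarm interaction into a prompt for LLM-driven NPC communication.
; InteractExecution validates its inputs, runs the parent interaction, then constructs and executes a BP_NPC_AlarmHearSignal for the instigator.
; If the signal succeeds, its prompt is wrapped in an NPC new-state prompt and sent through the StateManager's prompt manager with a set priority.
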(event EventBeginPlay
  (|CallParentFunction) ; This node is disabled and will not be called.\nDrag off pins to build functionality.
)

(event EventTick
  (params (DeltaSeconds :type Float%20%28single-precision%29)))

(fn InteractExecution
  (params (Instigator :type Actor%20Object%20Reference) (State%20Manager :type State%20Manager%20Object%20Reference))
  (if (and (Utilities|IsValid Instigator) (Utilities|IsValid State%20Manager))
    (|CallParentFunction Instigator State%20Manager)
    (bind _returnvalue (Game|ConstructObjectfromClass "/Game/LLMComunication/BP_NPC_AlarmHearSignal.BP_NPC_AlarmHearSignal_C" Instigator))
    (bind _returnvalue_2 (Class|LLMInteractionSignal|ExecuteSignal _returnvalue))
    (if _returnvalue_2
      (bind _returnvalue_3 (Class|LLMInteractionSignal|GetSignalPrompt _returnvalue))
      (bind _promp (Default|CreatePromp (Variables|/Game/LLMComunication/StateManager.StateManager_C|GetPrompManager State%20Manager) false false false true false (Utilities|Array|MakeArray _returnvalue_3)))
      (Default|SendPrompt (Variables|/Game/LLMComunication/StateManager.StateManager_C|GetPrompManager State%20Manager) _promp 1))))