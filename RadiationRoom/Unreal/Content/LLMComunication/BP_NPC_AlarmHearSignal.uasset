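; Alarm-hearing signal that turns nearby NPCs' awareness of a triggered alarm into LLM prompt text ordering them to chase the player.
; ExecuteSignal sphere-traces for Pawns within HearRange of the Instigator, ignoring it, and stores the hits.
; GetSignalPrompt casts hits to SimulationNPC, looks each up in its StateManager's Npcs map, appends an emergency line naming the Instigator, then prints and returns the prompt.
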(fn GetSignalPrompt
  (for _array_element (Variables|Default|GetHitResults)
    ;[1 1 1] Esto está feo, pero hasta que los NPC no tengan un componente de NPC es lo que hay
    (bind _assimulation_npc (Utilities|Casting|CastToSimulationNPC (.HitActor (Collision|BreakHitResult _array_element))))
    (if (.ReturnValue (Utilities|Map|Find (Variables|/Game/LLMComunication/StateManager.StateManager_C|GetNpcs (Variables|/Game/LLMComunication/SimulationNPC.SimulationNPC_C|GetStateManager _assimulation_npc)) (Variables|/Game/LLMComunication/SimulationNPC.SimulationNPC_C|GetNPCName _assimulation_npc)))
      (LocalVariables|SetReturnedPrompt (Utilities|String|Append (LocalVariables|GetReturnedPrompt) (.Value (Utilities|Map|Find (Variables|/Game/LLMComunication/StateManager.StateManager_C|GetNpcs (Variables|/Game/LLMComunication/SimulationNPC.SimulationNPC_C|GetStateManager _assimulation_npc)) (Variables|/Game/LLMComunication/SimulationNPC.SimulationNPC_C|GetNPCName _assimulation_npc))) " hears the allarm that was triggered by " (Utilities|GetDisplayName (Variables|Default|Getinstigator)) "You MUST chase the player, its an emergency"))))
  (Development|PrintString (LocalVariables|GetReturnedPrompt) true true "(R=0.216939,G=1.000000,B=0.000000,A=1.000000)")
  (return (LocalVariables|GetReturnedPrompt)))

(fn ExecuteSignal
  (bind _instigator (Variables|Default|Getinstigator))
  (bind _returnvalue (Transformation|GetActorLocation _instigator))
  (bind (_outhits _returnvalue_2) (Collision|MultiSphereTraceForObjects _returnvalue _returnvalue (Variables|Default|GetHearRange) (Utilities|Array|MakeArray "ObjectTypeQuery3") false (Utilities|Array|MakeArray (Variables|Default|Getinstigator)) "None"))
  (if _returnvalue_2
    (Variables|Default|SetHitResults _outhits)
    (return true)
    (else
      (return false))))