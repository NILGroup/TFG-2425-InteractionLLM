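; NPC sight signal that gathers nearby NPC data into a text prompt intended for an LLM.
; ExecuteSignal stores pawns found by a sphere trace within SightRange of the Instigator.
; GetSignalPrompt line-traces to each SimulationNPC as a rough visibility check, appending its StateManager entry by NPCName.
; The append runs when that trace reports a hit, although both endpoint actors are ignored, so it selects obstructed NPCs.
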(fn GetSignalPrompt
  (bind _instigator (Variables|Default|Getinstigator))
  (for _array_element (Variables|Default|GetHitResults)
    ;[1 1 1] Esto está feo, pero hasta que los NPC no tengan un componente de NPC es lo que hay
    (bind _assimulation_npc (Utilities|Casting|CastToSimulationNPC (.HitActor (Collision|BreakHitResult _array_element))))
    ;[1 1 1] Comprobación de que no hay nada entre el NPC y el jugador, no es una buena forma de comprobar la visibilidad, pero valdrá
    (bind _returnvalue (Collision|LineTraceByChannel (Transformation|GetActorLocation _instigator) (Transformation|GetActorLocation (.HitActor (Collision|BreakHitResult _array_element))) "TraceTypeQuery1" false (Utilities|Array|MakeArray (.HitActor (Collision|BreakHitResult _array_element)) _instigator) "None" true "(R=0.999918,G=1.000000,B=0.000000,A=1.000000)" "(R=1.000000,G=0.274615,B=0.000000,A=1.000000)"))
    (if _returnvalue
      (if (.ReturnValue (Utilities|Map|Find (Variables|/Game/LLMComunication/StateManager.StateManager_C|GetNpcs (Variables|/Game/LLMComunication/SimulationNPC.SimulationNPC_C|GetStateManager _assimulation_npc)) (Variables|/Game/LLMComunication/SimulationNPC.SimulationNPC_C|GetNPCName _assimulation_npc)))
        ;[1 0 0.1187] Hay que poner qué se le pasa al LLM
        (LocalVariables|SetReturnedPrompt (Utilities|String|Append (LocalVariables|GetReturnedPrompt) (.Value (Utilities|Map|Find (Variables|/Game/LLMComunication/StateManager.StateManager_C|GetNpcs (Variables|/Game/LLMComunication/SimulationNPC.SimulationNPC_C|GetStateManager _assimulation_npc)) (Variables|/Game/LLMComunication/SimulationNPC.SimulationNPC_C|GetNPCName _assimulation_npc))))))))
  (Development|PrintString (LocalVariables|GetReturnedPrompt) true true "(R=0.216939,G=1.000000,B=0.000000,A=1.000000)")
  (return (LocalVariables|GetReturnedPrompt)))

(fn ExecuteSignal
  (bind _instigator (Variables|Default|Getinstigator))
  (bind _returnvalue (Transformation|GetActorLocation _instigator))
  (bind (_outhits _returnvalue_2) (Collision|MultiSphereTraceForObjects _returnvalue _returnvalue (Variables|Default|GetSightRange) (Utilities|Array|MakeArray "ObjectTypeQuery3") false (Utilities|Array|MakeArray (Variables|Default|Getinstigator)) "None"))
  (if _returnvalue_2
    (Variables|Default|SetHitResults _outhits)
    (return true)
    (else
      (return false))))