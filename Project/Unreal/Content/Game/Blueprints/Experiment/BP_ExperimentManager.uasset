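; BP_ExperimentManager is an experiment manager that records participant user ID and group type to text files when play begins.
; On BeginPlay it sets the path to an Experiment folder under the project content directory, then fires the recording events.
; These create user_id.txt and group_type.txt if missing and write hardcoded values, ignoring the UserID and GroupType arguments passed in.
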(event EventBeginPlay
  (CallFunction|SetExperimentContentPath)
  (CallFunction|RSChangeUserInfo))

(event Custom|RSChangeUserInfo
  (params (UserID :type String) (GroupType :type String))
  (CallFunction|RSChangeUserID UserID)
  (CallFunction|RSChangeGroupType GroupType))

(event Custom|RSChangeGroupType
  (params (GroupType :type String))
  (Class|RRFileManager|CreateFileifNotExists (Variables|Default|GetExperimentContentPath) "group_type.txt")
  (Class|RRFileManager|WriteFileTXT (Variables|Default|GetExperimentContentPath) "group_type.txt" "CTRL"))

(event Custom|RSChangeUserID
  (params (UserID :type String))
  (Class|RRFileManager|CreateFileifNotExists (Variables|Default|GetExperimentContentPath) "user_id.txt")
  (Class|RRFileManager|WriteFileTXT (Variables|Default|GetExperimentContentPath) "user_id.txt" "CSN_BC"))

(fn ConstructionScript)

(fn SetExperimentContentPath
  (Variables|Default|SetExperimentContentPath (Utilities|String|Append (Class|KismetSystemLibrary|GetProjectContentDirectory) "/Experiment")))