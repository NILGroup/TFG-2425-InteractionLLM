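; Base NPC character with a name display, empty interact and cancel events, and a walk speed setter.
; On BeginPlay it caches the game instance, sets the name text and, after a short delay, sends an NPC event to the database only if it is a BP_NPC_Talkable.
; When CanLookPlayer is set, Tick yaws the capsule to face the player's follow camera.
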(event Custom|SetName
  (Rendering|Components|TextRender|SetText (Variables|Default|GetNPCName) (Utilities|Text|ToText(String) (Variables|NPCInfo|GetName))))

(event Custom|SendNPCToDB
  (bind _database_manager (CallFunction|GetMyDatabase))
  (Utilities|FlowControl|Delay 0.5)
  (bind _data (Default|GetDataBaseMainInfoEvent (CallFunction|GetMyGameInstance)))
  (Utilities|IsValid _database_manager
    (:Is%20Valid
      (Utilities|Casting|CastToBP_NPC_Talkable self)
      (Default|SendNPCtoDB _database_manager (Utilities|Struct|MakeF_NPCEvent 0 (.user_id (Utilities|Struct|BreakF_MainInfoEvent _data)) (.experiment_id (Utilities|Struct|BreakF_MainInfoEvent _data)) (.scenario_type (Utilities|Struct|BreakF_MainInfoEvent _data)) (Variables|NPCInfo|GetActorId) true)))
    (:Is%20Not%20Valid
      (Utilities|Casting|CastToBP_NPC_Talkable self)
      (Default|SendNPCtoDB _database_manager (Utilities|Struct|MakeF_NPCEvent 0 (.user_id (Utilities|Struct|BreakF_MainInfoEvent _data)) "" (.scenario_type (Utilities|Struct|BreakF_MainInfoEvent _data)) (Variables|NPCInfo|GetActorId))))))

(event Custom|LookAtPlayer
  ;[1 1 1] Look At Player
  (Transformation|SetWorldRotation (Variables|Collision|GetCapsuleComponent) (Math|Rotator|MakeRotator 0.0 0.0 (+ (.Yaw (Math|Rotator|BreakRotator (Math|Rotator|FindLookatRotation (Transformation|GetWorldLocation (Variables|/Game/Game/Blueprints/Player/BP_Player.BP_Player_C|GetFollowCamera (CallFunction|GetMyPlayer))) (Transformation|GetWorldLocation (Variables|Collision|GetCapsuleComponent))))) 1.8e+02)) false false))

(event EventBeginPlay
  (CallFunction|SendNPCtoDB)
  (bind _asrr_game_instance (Utilities|Casting|CastToRR_GameInstance (Game|GetGameInstance)))
  (Variables|Default|SetGameInstance _asrr_game_instance)
  (CallFunction|SetName))

(event EventInteractwith
  (params (Player :type BP%20Player%20Object%20Reference))
  ;[1 1 1] Interact
)

(event EventCancelInteract
  (params (Player :type BP%20Player%20Object%20Reference))
  ;[1 1 1] Interact
)

(event EventTick
  (params (DeltaSeconds :type Float%20%28single-precision%29))
  (Utilities|IsValid (CallFunction|GetMyPlayer)
    (:Is%20Valid
      (if (Variables|Player|GetCanLookPlayer)
        (CallFunction|LookatPlayer)))))

(fn ConstructionScript)

(fn UpdateWalkSpeed
  (params (Max%20Walk%20Speed :type Float%20%28double-precision%29))
  (Variables|/Script/Engine.CharacterMovementComponent|SetMaxWalkSpeed (Variables|Character|GetCharacterMovement) Max%20Walk%20Speed))