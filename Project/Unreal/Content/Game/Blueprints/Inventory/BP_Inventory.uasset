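; Backpack inventory actor whose slots are BP_InventoryItem child actors, registered and filled from data on BeginPlay.
; Opening and closing toggle slot interaction, fire dispatchers and log timestamped events to the experiment database via the game instance.
; Items spawned by slots enter a Tick-aged map that blocks putting them back until a timeout expires.
; Put-in checks also require an open inventory and reject slot targets, loaded clamps and one item type.
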(event Custom|RegisterToSpawnEvent
  (for _array_element (Variables|Default|GetInventoryItemList)
    (EventDispatchers|BindEventtoEDActorSpawned _array_element (delegate Custom|AddNewSpawnedItem))))

(event Custom|AddNewSpawnedItem
  (params (Actor :type BP%20Pickable%20Item%20Object%20Reference))
  (Utilities|Map|Add (Variables|Default|GetItemSpawnedTime) Actor 0.0))

(event Custom|SumTimeToItemSpawned
  (params (DeltaTime :type Float%20%28double-precision%29))
  (bind _keys (Utilities|Map|Keys (Variables|Default|GetItemSpawnedTime)))
  (for _array_element _keys
    (Utilities|Map|Add (Variables|Default|GetItemSpawnedTime) _array_element (+ (.Value (Utilities|Map|Find (Variables|Default|GetItemSpawnedTime) _array_element)) DeltaTime))))

(event Custom|RemoveItemSpawnedTime
  (bind _keys (Utilities|Map|Keys (Variables|Default|GetItemSpawnedTime)))
  (for _array_element _keys
    (if (>= (.Value (Utilities|Map|Find (Variables|Default|GetItemSpawnedTime) _array_element)) (Variables|Default|GetTimeToRemoveSpawnedItem))
      (Utilities|Map|Remove (Variables|Default|GetItemSpawnedTime) _array_element))))

(event Custom|InitInventoryItem
  (for _array_element (Components|GetChildrenComponents (Variables|Default|GetBackPack) false)
    (bind _aschild_actor_component (Utilities|Casting|CastToChildActorComponent _array_element))
    (bind _asbp_inventory_item (Utilities|Casting|CastToBP_InventoryItem (Variables|/Script/Engine.ChildActorComponent|GetChildActor _aschild_actor_component)))
    (Utilities|Array|Add (Variables|Default|GetInventoryItemList) _asbp_inventory_item)
    (Variables|/Game/Game/Blueprints/Inventory/BP_InventoryItem.BP_InventoryItem_C|SetInventory _asbp_inventory_item self)
    (Default|PutIteminbyData _asbp_inventory_item)
    (Variables|/Game/Game/Blueprints/Actors/Items/BP_ItemInitialState.BP_ItemInitialState_C|SetCanBeInteracted _asbp_inventory_item false)))

(event Custom|OpenInventory
  (CallFunction|SendInventoryEventtoDB 0 "NewEnumerator3")
  (Rendering|SetActorHiddenInGame false)
  (Variables|Default|SetIsOpen true)
  (Default|CallEDInventoryOpenned)
  (for _array_element (Variables|Default|GetInventoryItemList)
    (Variables|/Game/Game/Blueprints/Actors/Items/BP_ItemInitialState.BP_ItemInitialState_C|SetCanBeInteracted _array_element true)))

(event Custom|CloseInventory
  (CallFunction|SendInventoryEventtoDB 0 "NewEnumerator4")
  (Variables|Default|SetIsOpen false)
  (Default|CallEDInventoryClosed)
  (for _array_element (Variables|Default|GetInventoryItemList)
    (Variables|/Game/Game/Blueprints/Actors/Items/BP_ItemInitialState.BP_ItemInitialState_C|SetCanBeInteracted _array_element false)))

(event Custom|SendInventoryEventToDB
  (params (actor_id :type Integer) (event_type :type E_InventoryEventType%20Enum :default "NewEnumerator0") (actor_name :type String))
  (bind _data (Default|GetDataBaseMainInfoEvent (Variables|Default|GetGame%20Instance)))
  (bind _database_manager (Variables|/Game/Game/Blueprints/RR_GameInstance.RR_GameInstance_C|GetDatabase%20Manager (Variables|Default|GetGame%20Instance))
    (:then
      (Default|SendInventoryEventtoDB _database_manager (Utilities|Struct|MakeF_InventoryEvent 0 (.user_id (Utilities|Struct|BreakF_MainInfoEvent _data)) (.experiment_id (Utilities|Struct|BreakF_MainInfoEvent _data)) (.scenario_type (Utilities|Struct|BreakF_MainInfoEvent _data)) actor_id actor_name event_type (Math|DateTime|Now))))
    (:else)))

(event EventBeginPlay
  (bind _asrr_game_instance (Utilities|Casting|CastToRR_GameInstance (Game|GetGameInstance)))
  (Variables|Default|SetGame%20Instance _asrr_game_instance)
  (CallFunction|InitInventoryItem)
  (CallFunction|RegistertoSpawnEvent))

(event EventTick
  (params (DeltaSeconds :type Float%20%28single-precision%29))
  (CallFunction|SumTimetoItemSpawned DeltaSeconds)
  (CallFunction|RemoveItemSpawnedTime))

(fn ConstructionScript)

(fn CanPutItemInto?
  (params (Actor :type BP%20Pickable%20Item%20Object%20Reference))
  (if (Variables|Default|GetIsOpen)
    (for _array_element (Variables|Default|GetInventoryItemList)
      (if (== (Variables|/Game/Game/Blueprints/Inventory/BP_InventoryItem.BP_InventoryItem_C|GetTargetItem _array_element) Actor)
        (return false)))
    (bind _asbp_clamps (Utilities|Casting|CastToBP_Clamps Actor)
      (:then
        (if (Variables|/Game/Game/Blueprints/Actors/Items/UsableItems/BP_Clamps.BP_Clamps_C|GetHasItem _asbp_clamps)
          (return false)
          (else
            _)))
      (:CastFailed
        _))
    (return (and (not (.ReturnValue (Utilities|Map|Find (Variables|Default|GetItemSpawnedTime) Actor))) (Utilities|Enum|NotEqual(Enum) (Variables|/Game/Game/Blueprints/Actors/Items/BP_InteractItemParent.BP_InteractItemParent_C|GetItemType Actor) "NewEnumerator11")))
    (else
      (return false))))

(fn CanTakeOut?
  (return (Variables|Default|GetIsOpen)))