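; Gameplay manager for the T1 tutorial scenario, extending a parent manager with a linear chain of five quests.
; A Tuddy intro dialog and welcome countdown teleport the player to the start and begin the first quest.
; Player, item, place-point and NPC events advance quests through teleporting, detecting, grabbing, placing and conversation, stepping the tutorial display.
; After completion, an end trigger starts Tuddy's closing dialog, then a goodbye countdown ends gameplay.
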(event EventBeginPlay
  (|CallParentFunction)
  (Utilities|FlowControl|Sequence
    (:then_0
      (Variables|Default|SetCanStartCurrentQuest false))
    (:then_1
      (Rendering|SetActorHiddenInGame (Variables|Default|GetGoodbyeWidget) true))))

(event EventStartScenario
  (bind _starttuddy (Variables|Tuddy|GetStartTuddy))
  (|CallParentFunction)
  (Default|Show _starttuddy)
  (Utilities|FlowControl|Delay 0.5)
  (Default|StartNewDialogbyID (Variables|/Game/Game/Blueprints/Tutorial/BP_TutorialBuddy.BP_TutorialBuddy_C|GetAC_TuddyDialogManager _starttuddy) "T1001"))

(event EventCompleteQuest
  (params (QuestID :type Name :default "None"))
  (|CallParentFunction QuestID)
  (Variables|Default|SetCanStartCurrentQuest false)
  (Default|NextDisplay (Variables|Default|GetTutorialDisplayManager))
  (if (Variables|Default|GetGameplayCompleted)
    (Utilities|FlowControl|Delay 1.0)
    (Default|Show (Variables|Tuddy|GetEndTuddy))
    (Rendering|SetActorHiddenInGame (Variables|Default|GetGoodbyeWidget) false)))

(event Custom|OnGoodbyeCountdownCompleted
  (CallFunction|EndGameplay))

(event Custom|OnStartTuddyDialogCompleted
  (params (CurrentTuddyDialogType :type E_TuddyDialogLinesType%20Enum :default "NewEnumerator0") (CurrentExtraLineType :type E_TuddyExtraLineTypes%20Enum :default "NewEnumerator1") (DialogID :type Name))
  (bind _welcomewidget (Variables|Default|GetWelcomeWidget))
  (Default|Hide (Variables|Tuddy|GetStartTuddy))
  (Rendering|SetActorHiddenInGame (Variables|Default|GetWelcomeWidget) false)
  (Default|StartCountdown _welcomewidget)
  (EventDispatchers|BindEventtoEDCountdownEnded _welcomewidget (delegate Custom|OnWelcomeCountdownCompleted)))

(event Custom|OnEndTuddyDialogCompleted
  (params (CurrentTuddyDialogType :type E_TuddyDialogLinesType%20Enum :default "NewEnumerator0") (CurrentExtraLineType :type E_TuddyExtraLineTypes%20Enum :default "NewEnumerator1") (DialogID :type Name))
  (bind _goodbyewidget (Variables|Default|GetGoodbyeWidget))
  (Default|Hide (Variables|Tuddy|GetEndTuddy))
  (Rendering|SetActorHiddenInGame (Variables|Default|GetGoodbyeWidget) false)
  (Default|StartCountdown _goodbyewidget)
  (EventDispatchers|BindEventtoEDCountdownEnded _goodbyewidget (delegate Custom|OnGoodbyeCountdownCompleted)))

(event Custom|OnWelcomeCountdownCompleted
  (Transformation|SetActorLocation (CallFunction|GetMyPlayer) (Transformation|GetActorLocation (Variables|Default|GetInitialTeleportPoint)) false true)
  (CallFunction|SetCurrentQuest "T1001")
  (Default|StartFirstDisplay (Variables|Default|GetTutorialDisplayManager)))

(event EventBindTuddyActions
  (|CallParentFunction)
  (EventDispatchers|BindEventtoEDDialogCompleted (Variables|/Game/Game/Blueprints/Tutorial/BP_TutorialBuddy.BP_TutorialBuddy_C|GetAC_TuddyDialogManager (Variables|Tuddy|GetStartTuddy)) (delegate Custom|OnStartTuddyDialogCompleted))
  (EventDispatchers|BindEventtoEDDialogCompleted (Variables|/Game/Game/Blueprints/Tutorial/BP_TutorialBuddy.BP_TutorialBuddy_C|GetAC_TuddyDialogManager (Variables|Tuddy|GetEndTuddy)) (delegate Custom|OnEndTuddyDialogCompleted)))

(event Custom|OnActorOverlapEndTrigger
  (params (OverlappedActor :type Actor%20Object%20Reference) (OtherActor :type Actor%20Object%20Reference))
  (if (== OtherActor (CallFunction|GetMyPlayer))
    (if (Variables|Default|GetGameplayCompleted)
      (Default|StartNewDialogbyID (Variables|/Game/Game/Blueprints/Tutorial/BP_TutorialBuddy.BP_TutorialBuddy_C|GetAC_TuddyDialogManager (Variables|Tuddy|GetEndTuddy)) "T1002"))))

(event Custom|OnPlayerTeleported
  (if (CallFunction|IsCurrentQuestandCanStart "T1001")
    (bind _output_get (Variables|Counters|SetTimesTeleported (+ (Variables|Counters|GetTimesTeleported) 1)))
    (if (== _output_get 5)
      (CallFunction|CompleteQuest (Variables|Default|GetCurrentQuestID))
      (CallFunction|SetCurrentQuest "T1002"))))

(event EventBindPlayerActions
  (|CallParentFunction)
  (EventDispatchers|BindEventtoEDTeleported (CallFunction|GetMyPlayer) (delegate Custom|OnPlayerTeleported))
  (Collision|BindEventtoOnActorBeginOverlap (Variables|Default|GetEndTrigger) (delegate Custom|OnActorOverlapEndTrigger)))

(event Custom|OnTutorialItemDetected
  (params (Actor :type BP%20Interact%20Item%20Parent%20Object%20Reference))
  (bind _detectedactors (Variables|Counters|GetDetectedActors))
  (if (CallFunction|IsCurrentQuestandCanStart "T1002")
    (if (not (Utilities|Array|ContainsItem _detectedactors Actor))
      (bind _returnvalue (Utilities|Array|Add _detectedactors Actor))
      (if (== _returnvalue (- (Variables|Counters|GetMaxDetectedActors) 1))
        (CallFunction|CompleteQuest (Variables|Default|GetCurrentQuestID))
        (CallFunction|SetCurrentQuest "T1003")))))

(event Custom|OnTutorialItemGrabbed
  (params (Actor :type BP%20Interact%20Item%20Parent%20Object%20Reference))
  (bind _grabbedactors (Variables|Counters|GetGrabbedActors))
  (if (CallFunction|IsCurrentQuestandCanStart "T1003")
    (if (not (Utilities|Array|ContainsItem _grabbedactors Actor))
      (bind _returnvalue (Utilities|Array|Add _grabbedactors Actor))
      (if (== _returnvalue (- (Variables|Counters|GetMaxGrabbedActors) 1))
        (CallFunction|CompleteQuest (Variables|Default|GetCurrentQuestID))
        (CallFunction|SetCurrentQuest "T1004")))))

(event Custom|OnPlacePointManagerCompleted
  (if (CallFunction|IsCurrentQuestandCanStart "T1004")
    (if (CallFunction|AllPlacePointManagersCompleted)
      (CallFunction|CompleteQuest (Variables|Default|GetCurrentQuestID))
      (CallFunction|SetCurrentQuest "T1005"))))

(event EventBindItemActions
  (|CallParentFunction)
  (bind _outactors (Actor|GetAllActorsOfClass "/Game/Game/Blueprints/Actors/Items/BP_PickableItem.BP_PickableItem_C"))
  (bind _output_get (Variables|Default|SetPickableItemsList _outactors))
  (for _array_element _output_get
    (EventDispatchers|BindEventtoEDDetectionStarted _array_element (delegate Custom|OnTutorialItemDetected))
    (EventDispatchers|AssignEDInteractionStarted _array_element (delegate Custom|OnTutorialItemGrabbed))))

(event EventBindPlacePointsActions
  (|CallParentFunction)
  (for _array_element (Variables|Default|GetPlacePointManagers)
    (Variables|/Game/Game/Blueprints/Actors/Items/PlacePoints/BP_PlacePointManager.BP_PlacePointManager_C|SetCanActivatePoints _array_element false)
    (EventDispatchers|BindEventtoEDAllPlacePointswithItems _array_element (delegate Custom|OnPlacePointManagerCompleted))))

(event Custom|OnNPCConversationFinished
  (params (ConversationNumber :type Integer))
  (if (CallFunction|IsCurrentQuestandCanStart "T1005")
    (CallFunction|CompleteQuest (Variables|Default|GetCurrentQuestID))
    (Default|NextConversation (Variables|Default|GetNPC))))

(event EventBindNPCActions
  (|CallParentFunction)
  (bind _npc (Variables|Default|GetNPC)
    (:then
      (EventDispatchers|BindEventtoEDConversationFinished _npc (delegate Custom|OnNPCConversationFinished)))
    (:else
      (Default|Log (CallFunction|GetMyGameInstance) "NewEnumerator2" "Falta NPC" false))))

(fn ConstructionScript)

(fn AllPlacePointManagersCompleted
  (for _array_element (Variables|Default|GetPlacePointManagers)
    (if (not (Variables|/Game/Game/Blueprints/Actors/Items/PlacePoints/BP_PlacePointManager.BP_PlacePointManager_C|GetAllPointsUsed _array_element))
      (return false)))
  (return true))