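; Radiation shielding area actor that applies a material's attenuation to actors inside it.
; On BeginPlay it searches the shields data table for its configured material and caches that row's attenuation coefficient.
; Begin overlap passes the shielding data and shield thickness to the other actor's AC_Radiation component, and end overlap tells that component it has left the zone.
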(event Custom|SetShieldData
  (bind _shieldsdatatable (Variables|Default|GetShieldsDataTable))
  (bind _outrownames (DataTable|GetDataTableRowNames _shieldsdatatable))
  (bind _array_element (Utilities|Array|ForEachLoopwithBreak _outrownames :!label _label)
    (:LoopBody
      (bind _returnvalue (Utilities|GetDataTableRow _shieldsdatatable _array_element)
        (:then
          (if (Utilities|Enum|Equal(Enum) (.Material (Utilities|Struct|BreakF_ShieldingMaterialData _returnvalue)) (.Material (Utilities|Struct|BreakF_ShieldingMaterialData (Variables|Default|GetShieding%20Material%20Data))))
            (Variables|Default|SetShieding%20Material%20Data (Utilities|Struct|MakeF_ShieldingMaterialData (.Material (Utilities|Struct|BreakF_ShieldingMaterialData _returnvalue)) (.AttenuationCoefficient (Utilities|Struct|BreakF_ShieldingMaterialData _returnvalue))))
            (goto _label Break)))))))

(event EventBeginPlay
  (CallFunction|SetShieldData))

(event Collision|EventActorBeginOverlap
  (params (OtherActor :type Actor%20Object%20Reference))
  (Default|EntertoAttenuationZone (Actor|GetComponentbyClass OtherActor "/Game/Game/Blueprints/Components/AC_Radiation.AC_Radiation_C") (Variables|Default|GetShieding%20Material%20Data) (Variables|Default|GetShieldThickness)))

(event Collision|EventActorEndOverlap
  (params (OtherActor :type Actor%20Object%20Reference))
  (Default|ExitOfAttenuationZone (Actor|GetComponentbyClass OtherActor "/Game/Game/Blueprints/Components/AC_Radiation.AC_Radiation_C")))

(fn ConstructionScript)