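; RBQ van actor that spawns items requested through its child RBQ panel and logs the panel's activity to the database.
; Panel increase, decrease and spawn events become timestamped RBQ records tagged with user, experiment and scenario.
; Item types resolve to IDs and data through a data table scan.
; Spawning scatters item actors at random points just above the Plane's bounds, initializes each from its data and broadcasts per-item and per-type notifications.
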(event Custom|OnItemIncrease
  (params (ItemType :type E_ItemType%20Enum :default "NewEnumerator2") (Count :type Integer))
  (bind _listofids (CallFunction|GetItemsIds (Utilities|Array|MakeArray ItemType)))
  (CallFunction|SendRBQEventtoDB "NewEnumerator0" _listofids (Utilities|Array|MakeArray Count)))

(event Custom|SendRBQEventToDB
  (params (event_type :type E_RBQEventType%20Enum :default "NewEnumerator0") (actor_id :type Array%20of%20Integers) (num_of_actors :type Array%20of%20Integers))
  (bind _database_manager (CallFunction|GetMyDatabase))
  (bind _data (Default|GetDataBaseMainInfoEvent (CallFunction|GetMyGameInstance)))
  (Utilities|IsValid _database_manager
    (:Is%20Valid
      (Default|SendRBQEventtoDB _database_manager (Utilities|Struct|MakeF_RBQEvent 0 (.user_id (Utilities|Struct|BreakF_MainInfoEvent _data)) (.experiment_id (Utilities|Struct|BreakF_MainInfoEvent _data)) (.scenario_type (Utilities|Struct|BreakF_MainInfoEvent _data)) event_type actor_id num_of_actors (Math|DateTime|Now))))))

(event Custom|OnItemDecrease
  (params (ItemType :type E_ItemType%20Enum :default "NewEnumerator2") (Count :type Integer))
  (bind _listofids (CallFunction|GetItemsIds (Utilities|Array|MakeArray ItemType)))
  (CallFunction|SendRBQEventtoDB "NewEnumerator1" _listofids (Utilities|Array|MakeArray Count)))

(event Custom|SpawnItems
  (params (Items :type Map%20of%20E_ItemType%20Enums%20to%20Integers :default "NewEnumerator2"))
  (bind _plane (Variables|Default|GetPlane))
  (bind (_origin _boxextent) (Collision|GetComponentBounds _plane))
  (Utilities|FlowControl|Sequence
    (:then_0
      (bind _keys (Utilities|Map|Keys Items))
      (bind _listofids (CallFunction|GetItemsIds _keys))
      (bind _values (Utilities|Map|Values Items))
      (CallFunction|SendRBQEventtoDB "NewEnumerator2" _values _listofids))
    (:then_1
      (bind _keys_2 (Utilities|Map|Keys Items))
      (for _array_element _keys_2
        (bind _auxitemdata (CallFunction|GetItemDatatoSpawn _array_element))
        (if (.ReturnValue (Utilities|Map|Find Items _array_element))
          (for _index (range 0 (- (.Value (Utilities|Map|Find Items _array_element)) 1))
            (bind _returnvalue (Game|SpawnActorfromClass "/Game/Game/Blueprints/Actors/Items/BP_ItemInitialState.BP_ItemInitialState_C" (Math|Transform|MakeTransform (+ (Math|Random|RandomPointinBoundingBox _origin _boxextent) "0.000000,0.000000,20.000000")) "AdjustIfPossibleButAlwaysSpawn" "MultiplyWithRoot" 0 0))
            (Default|PutIteminbyData _returnvalue _auxitemdata)
            (Default|CallEDItemSpawned _returnvalue))
          (Default|CallEDMultipleItemsSpawned _array_element (.Value (Utilities|Map|Find Items _array_element))))))))

(event EventBeginPlay
  (Utilities|FlowControl|Sequence
    (:then_0
      (bind _asbp_rbqpanel_actor (Utilities|Casting|CastToBP_RBQPanelActor (Variables|/Script/Engine.ChildActorComponent|GetChildActor (Variables|Default|GetChildActor))))
      (Variables|Default|SetRBQPanel%20Actor _asbp_rbqpanel_actor))
    (:then_1
      (EventDispatchers|BindEventtoEDIncreaseItem (Variables|Default|GetRBQPanel%20Actor) (delegate Custom|OnItemIncrease))
      (EventDispatchers|BindEventtoEDDecreaseItem (Variables|Default|GetRBQPanel%20Actor) (delegate Custom|OnItemDecrease))
      (EventDispatchers|BindEventtoEDSpawnItems (Variables|Default|GetRBQPanel%20Actor) (delegate Custom|SpawnItems)))))

(fn ConstructionScript)

(fn GetItemDatatoSpawn
  (params (ItemType :type E_ItemType%20Enum :default "NewEnumerator2"))
  (bind _itemdata_datatable (Variables|SpawnItems|GetItemData%20Datatable))
  (bind _outrownames (DataTable|GetDataTableRowNames _itemdata_datatable))
  (for _array_element _outrownames
    (bind _returnvalue (Utilities|GetDataTableRow _itemdata_datatable _array_element)
      (:then
        (if (Utilities|Enum|Equal(Enum) (.Type (Utilities|Struct|BreakF_ItemData _returnvalue)) ItemType)
          (return _returnvalue))))))

(fn GetItemsIds
  (params (ItemTypes :type Array%20of%20E_ItemType%20Enums :default "NewEnumerator2"))
  (for _array_element ItemTypes
    (bind _auxitemdata (CallFunction|GetItemDatatoSpawn _array_element))
    (Utilities|Array|Add (LocalVariables|GetAuxList) (.Id (Utilities|Struct|BreakF_ItemData _auxitemdata))))
  (return (LocalVariables|GetAuxList)))