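; Tutorial variant of a pickable item that reports the player's detection and grab actions through event dispatchers.
; It extends the parent's detection and interaction events, recording detected and grabbed states when allowed.
; A Liar flag changes the grab type, reveals a widget on detection and suppresses the grab notification.
; Spawn plays a pop sound, then after a short delay unhides the item and enables physics and interaction.
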(event Custom|Spawn
  (Audio|PlaySoundatLocation "/Game/Game/Assets/Sounds/effects/cartoon_pop.cartoon_pop" (Transformation|GetWorldLocation (Variables|Default|GetStaticMesh)) "0, 0, 0" 1.0 1.0 0.0 0 0 0 0)
  (Utilities|FlowControl|Delay 0.2)
  (Rendering|SetActorHiddenInGame false)
  (Physics|SetSimulatePhysics (Variables|Default|GetStaticMesh) true)
  (Variables|Default|SetCanBeInteracted true))

(event EventBeginPlay
  (|CallParentFunction)
  (if (Variables|Default|GetLiar)
    (Variables|/Game/VRTemplate/Blueprints/GrabComponent.GrabComponent_C|SetGrabType (Variables|Default|GetGrabComponent) "NewEnumerator0")))

(event EventCancelInteract
  (params (Player :type BP%20Player%20Object%20Reference) (Hand :type EControllerHand%20Enum :default "Left"))
  (|CallParentFunction Player "Left")
  (Physics|SetSimulatePhysics (Variables|Default|GetStaticMesh) true))

(event EventStopDetection
  (params (Player :type BP%20Player%20Object%20Reference) (Hand :type EControllerHand%20Enum :default "Left"))
  (|CallParentFunction Player "Left"))

(event EventStartDetection
  (params (Player :type BP%20Player%20Object%20Reference) (Hand :type EControllerHand%20Enum :default "Left"))
  (|CallParentFunction Player "Left")
  (if (Variables|Default|GetCanBeDetected)
    (Variables|Default|SetHasBeenDetected true)
    (Default|CallEDDetectionStarted)
    (if (Variables|Default|GetLiar)
      (Development|SetHiddeninGame (Variables|Default|GetWidget) false false))))

(event EventInteractwith
  (params (Player :type BP%20Player%20Object%20Reference) (Hand :type EControllerHand%20Enum :default "Left"))
  (|CallParentFunction Player "Left")
  (if (and (not (Variables|Default|GetLiar)) (Variables|Default|GetCanBeGrabbed))
    (Variables|Default|SetHasBeenGrabbed true)
    (Default|CallEDInteractionStarted)))

(fn ConstructionScript
  (|CallParentFunction))