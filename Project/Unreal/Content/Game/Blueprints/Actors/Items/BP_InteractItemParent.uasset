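; Base actor for interactable items, with radiation contamination and experiment database logging.
; Interaction and detection events fire event dispatchers, and a mesh hit from an actor with a radiation component marks the item contaminated.
; It registers itself with the database shortly after BeginPlay, tagged with user, experiment and scenario info from the GameInstance.
; A helper logs interaction events; the final-event flush on database close is an empty stub here.
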(event OnComponentHit(StaticMesh)
  (params (HitComponent :type Primitive%20Component%20Object%20Reference) (OtherActor :type Actor%20Object%20Reference) (OtherComp :type Primitive%20Component%20Object%20Reference) (NormalImpulse :type Vector :default "0, 0, 0") (Hit :type Hit%20Result%20Structure%20%28by%20ref%29))
  (Utilities|IsValid (Actor|GetComponentbyClass OtherActor "/Game/Game/Components/AC_Radiation.AC_Radiation_C")
    (:Is%20Valid
      (Variables|/Game/Game/Components/AC_Radiation.AC_Radiation_C|SetIsContamined? (Variables|Default|GetAC_Radiation) true))))

(event EventBeginPlay
  (|CallParentFunction)
  (CallFunction|BindDatabaseEvents)
  (CallFunction|SendItemtoDB))

(event EventInteractwith
  (params (Player :type BP%20Player%20Object%20Reference) (Hand :type EControllerHand%20Enum :default "Left"))
  ;[1 1 1] Interact
  (Default|CallEDInteractionStarted self))

(event EventCancelInteract
  (params (Player :type BP%20Player%20Object%20Reference) (Hand :type EControllerHand%20Enum :default "Left"))
  ;[1 1 1] Interact
  (Default|CallEDInteractionCompleted self))

(event EventTick
  (params (DeltaSeconds :type Float%20%28single-precision%29)))

(event EventStartDetection
  (params (Player :type BP%20Player%20Object%20Reference) (Hand :type EControllerHand%20Enum :default "Left"))
  ;[1 1 1] Detection
  (Default|CallEDDetectionStarted self))

(event EventStopDetection
  (params (Player :type BP%20Player%20Object%20Reference) (Hand :type EControllerHand%20Enum :default "Left"))
  ;[1 1 1] Detection
  (Default|CallEDDetectionCompleted self))

(event Custom|SendInteractEventToDB
  (params (EventType :type E_ItemEventType%20Enum :default "NewEnumerator4") (hand :type EControllerHand%20Enum :default "Left") (event_datetime :type Date%20Time%20Structure))
  (bind _database_manager (CallFunction|GetMyDatabase))
  (bind _data (Default|GetDataBaseMainInfoEvent (CallFunction|GetMyGameInstance)))
  (Utilities|IsValid _database_manager
    (:Is%20Valid
      (Default|SendItemInteractionEventtoDB _database_manager (Utilities|Struct|MakeF_ItemInteractionEvent 0 (.user_id (Utilities|Struct|BreakF_MainInfoEvent _data)) (.experiment_id (Utilities|Struct|BreakF_MainInfoEvent _data)) (.scenario_type (Utilities|Struct|BreakF_MainInfoEvent _data)) (Variables|ItemInfo|GetActorId) (Utilities|GetDisplayName self) EventType hand event_datetime)))))

(event Custom|BindDatabaseEvents
  (EventDispatchers|AssignEDDatabaseNeedtobeClosed (Variables|Default|GetAC_Database) (delegate Custom|OnDatabaseNeedToBeClosed))
  (EventDispatchers|AssignEDDatabaseClosed (Variables|Default|GetAC_Database) (delegate Custom|OnDatabaseClosed)))

(event Custom|OnDatabaseNeedToBeClosed
  (CallFunction|SendLastEventstoDB))

(event Custom|OnDatabaseClosed)

(event Custom|SendLastEventsToDB)

(event Custom|SendItemToDB
  (bind _database_manager (CallFunction|GetMyDatabase))
  (Utilities|FlowControl|Delay 0.5)
  (bind _data (Default|GetDataBaseMainInfoEvent (CallFunction|GetMyGameInstance)))
  (Utilities|IsValid _database_manager
    (:Is%20Valid
      (Default|SendItemtoDB _database_manager (Utilities|Struct|MakeF_ItemEvent 0 (.user_id (Utilities|Struct|BreakF_MainInfoEvent _data)) (.experiment_id (Utilities|Struct|BreakF_MainInfoEvent _data)) (.scenario_type (Utilities|Struct|BreakF_MainInfoEvent _data)) (Variables|ItemInfo|GetActorId) (Utilities|GetDisplayName self))))))

(fn ConstructionScript)