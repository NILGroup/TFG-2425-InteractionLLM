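; Actor component that links its owner to the database for logging radiation exposure events from the player and EPD dosimeters.
; On BeginPlay it binds to the database's close-request and closed dispatchers and re-broadcasts them through its own.
; Send events pack the owner's dose rate, absorption, position and time arrays with Game Instance user, experiment and scenario info.
; Player events are sent only when a radiation emission point exists in the level.
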(event Custom|BindDatabaseEvents
  (bind _database_manager (CallFunction|GetMyDatabase))
  (Utilities|IsValid _database_manager
    (:Is%20Valid
      (EventDispatchers|AssignEDDatabaseNeedtobeClosed _database_manager (delegate Custom|OnDatabaseNeedToBeClosed))
      (EventDispatchers|AssignEDDatabaseClosed _database_manager (delegate Custom|OnDatabaseClosed)))))

(event Custom|OnDatabaseNeedToBeClosed
  (Default|CallEDDatabaseNeedtobeClosed))

(event Custom|OnDatabaseClosed
  (Default|CallEDDatabaseClosed))

(event EventBeginPlay
  (Variables|Default|SetOwner (Components|GetOwner))
  (CallFunction|BindDatabaseEvents))

(event Custom|SendEPDRadiationEventToDB
  (bind _database_manager (CallFunction|GetMyDatabase))
  (bind _data (Default|GetDataBaseMainInfoEvent (CallFunction|GetMyGameInstance)))
  (bind _asbp_dosimeter_epd (Utilities|Casting|CastToBP_Dosimeter_EPD (Variables|Default|GetOwner)))
  (Utilities|IsValid _database_manager
    (:Is%20Valid
      (Default|SendEPDRadiationEventtoDB _database_manager (Utilities|Struct|MakeF_EPDRadiationEvent 0 (.user_id (Utilities|Struct|BreakF_MainInfoEvent _data)) (.experiment_id (Utilities|Struct|BreakF_MainInfoEvent _data)) (.scenario_type (Utilities|Struct|BreakF_MainInfoEvent _data)) (Variables|/Game/Game/Blueprints/Actors/Dosimeters/BP_Dosimeter_EPD.BP_Dosimeter_EPD_C|GetEPDId _asbp_dosimeter_epd) (Variables|/Game/Game/Blueprints/Actors/Dosimeters/BP_Dosimeter_EPD.BP_Dosimeter_EPD_C|GetCurrentEventDoseRateArray _asbp_dosimeter_epd) (Variables|/Game/Game/Blueprints/Actors/Dosimeters/BP_Dosimeter_EPD.BP_Dosimeter_EPD_C|GetCurrentEventDoseAbsortionArray _asbp_dosimeter_epd) (Variables|/Game/Game/Blueprints/Actors/Dosimeters/BP_Dosimeter_EPD.BP_Dosimeter_EPD_C|GetCurrentEventPositionArray _asbp_dosimeter_epd) (Variables|/Game/Game/Blueprints/Actors/Dosimeters/BP_Dosimeter_EPD.BP_Dosimeter_EPD_C|GetCurrentEventDatetimeArray _asbp_dosimeter_epd))))))

(event Custom|SendUserRadiationEventToDB
  (bind _database_manager (CallFunction|GetMyDatabase))
  (bind _returnvalue (Actor|GetActorOfClass "/Game/Game/Blueprints/Actors/Radiation/BP_RadiationEmissionPoint.BP_RadiationEmissionPoint_C"))
  (Utilities|IsValid _returnvalue
    (:Is%20Valid
      (bind _data (Default|GetDataBaseMainInfoEvent (CallFunction|GetMyGameInstance)))
      (bind _asbp_player (Utilities|Casting|CastToBP_Player (Variables|Default|GetOwner)))
      (Utilities|IsValid _database_manager
        (:Is%20Valid
          (Default|SendUserRadiationEventtoDB _database_manager (Utilities|Struct|MakeF_UserRadiationEvent 0 (.user_id (Utilities|Struct|BreakF_MainInfoEvent _data)) (.experiment_id (Utilities|Struct|BreakF_MainInfoEvent _data)) (.scenario_type (Utilities|Struct|BreakF_MainInfoEvent _data)) (Variables|/Game/Game/Blueprints/Player/BP_Player.BP_Player_C|GetCurrentEventRadiationDoseRateArray _asbp_player) (Variables|/Game/Game/Blueprints/Player/BP_Player.BP_Player_C|GetCurrentEventDoseRadiationAbsortionArray _asbp_player) (Variables|/Game/Game/Blueprints/Player/BP_Player.BP_Player_C|GetCurrentEventRadiationPositionArray _asbp_player) (Variables|/Game/Game/Blueprints/Player/BP_Player.BP_Player_C|GetCurrentEventRadiationDatetimeArray _asbp_player))))))))