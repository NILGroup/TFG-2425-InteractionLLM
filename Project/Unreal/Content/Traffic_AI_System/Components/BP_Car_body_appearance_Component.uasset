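; Traffic AI vehicle component that manages car body appearance: lights, paint, dirt and doors.
; On BeginPlay it spawns shadowless front and rear spotlights with light functions from mesh bounds, and creates dynamic materials for "Lights" and "Body" slots, randomizing color and dirtiness.
; Events toggle indicators, hazards, headlights, brake and reverse lights through material parameters, with headlights and brakes also setting spotlight intensity.
; OpenDoor passes door states to ABP_Traffic_Car on skeletal meshes.
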(event Custom|Set%20up%20car%20body
  (params (Owner :type Actor%20Object%20Reference) (Car%20Body :type Mesh%20Component%20Object%20Reference))
  (bind _car_colors (Variables|Color|GetCar%20Colors))
  (bind _returnvalue (Utilities|Array|LastIndex _car_colors))
  (Utilities|FlowControl|Sequence
    (:then_0
      (Variables|System|SetOwner Owner)
      (Variables|Default|SetCar%20Body%20mesh Car%20Body))
    (:then_1
      ;[1 0.7401 0.4135] Add head light (one spot light with light function)
      (bind _asskeletal_mesh_component (Utilities|Casting|CastToSkeletalMeshComponent (Variables|Default|GetCar%20Body%20mesh)) ; Pure cast changed to impure cast in 1.2 to avoid errors when using static mesh as a root component
        (:then
          (Variables|Default|SetRelative%20transform%20X (+ (.X (Math|Vector|BreakVector (.origin (Class|SkeletalMesh|GetImportedBounds (Variables|/Script/Engine.SkinnedMeshComponent|GetSkeletalMesh _asskeletal_mesh_component))))) (.x (.boxextent (Class|SkeletalMesh|GetImportedBounds (Variables|/Script/Engine.SkinnedMeshComponent|GetSkeletalMesh _asskeletal_mesh_component)))))))
        (:CastFailed
          (bind _asstatic_mesh_component (Utilities|Casting|CastToStaticMeshComponent (Variables|Default|GetCar%20Body%20mesh)))
          (Variables|Default|SetRelative%20transform%20X (.SphereRadius (Collision|GetComponentBounds _asstatic_mesh_component)))))
      (bind _returnvalue_2 (Game|AddComponentbyClass (Variables|System|GetOwner) "/Script/Engine.SpotLightComponent" false (Math|Transform|MakeTransform (Math|Vector|MakeVector (Variables|Default|GetRelative%20transform%20X) 0.0 (Variables|Lights|GetFront%20light%20Z%20offset)) "-10.000000, 0,0.000000" "1,1,1")))
      (Rendering|Components|Light|SetCastShadows _returnvalue_2 false)
      (Rendering|Components|Light|SetIntensity _returnvalue_2 (Variables|Lights|GetFront%20Light%20intensity))
      (Rendering|Components|Light|SetLightColor _returnvalue_2 (Variables|Lights|GetFront%20light%20color) true)
      (Rendering|Lighting|SetAttenuationRadius _returnvalue_2 (Variables|Lights|GetFront%20light%20radius))
      (Rendering|Lighting|SetOuterConeAngle _returnvalue_2 (Variables|Lights|GetFront%20light%20Outer%20Cone%20Angle))
      (Rendering|Components|Light|SetLightFunctionMaterial _returnvalue_2 (Variables|Lights|GetFront%20light%20material%20function))
      (Variables|Default|SetFront%20light _returnvalue_2))
    (:then_2
      ;[1 0.1668 0.06708] Add tail light (one spot light with light function)
      (bind _asskeletal_mesh_component_2 (Utilities|Casting|CastToSkeletalMeshComponent (Variables|Default|GetCar%20Body%20mesh)) ; Pure cast changed to impure cast in 1.2 to avoid errors when using static mesh as a root component
        (:then
          (Variables|Default|SetRelative%20transform%20X (- (.x (.boxextent (Class|SkeletalMesh|GetImportedBounds (Variables|/Script/Engine.SkinnedMeshComponent|GetSkeletalMesh _asskeletal_mesh_component_2)))) (.X (Math|Vector|BreakVector (.origin (Class|SkeletalMesh|GetImportedBounds (Variables|/Script/Engine.SkinnedMeshComponent|GetSkeletalMesh _asskeletal_mesh_component_2))))))))
        (:CastFailed
          (bind _asstatic_mesh_component_2 (Utilities|Casting|CastToStaticMeshComponent (Variables|Default|GetCar%20Body%20mesh)))
          (Variables|Default|SetRelative%20transform%20X (.SphereRadius (Collision|GetComponentBounds _asstatic_mesh_component_2)))))
      (bind _returnvalue_3 (Game|AddComponentbyClass (Variables|System|GetOwner) "/Script/Engine.SpotLightComponent" false (Math|Transform|MakeTransform (Math|Vector|MakeVector (* (Variables|Default|GetRelative%20transform%20X) -1.0) 0.0 (Variables|Lights|GetRear%20light%20Z%20offset)) "0,180.000000, 0" "1,1,1")))
      (Rendering|Components|Light|SetCastShadows _returnvalue_3 false)
      (Rendering|Components|Light|SetIntensity _returnvalue_3 (Variables|Lights|GetRear%20light%20intencity))
      (Rendering|Components|Light|SetLightColor _returnvalue_3 (Variables|Lights|GetRear%20light%20color) true)
      (Rendering|Lighting|SetAttenuationRadius _returnvalue_3 (Variables|Lights|GetRear%20light%20radius))
      (Rendering|Lighting|SetOuterConeAngle _returnvalue_3 (Variables|Lights|GetRear%20light%20angle))
      (Rendering|Components|Light|SetLightFunctionMaterial _returnvalue_3 (Variables|Lights|GetRear%20light%20material%20function))
      (Variables|Default|SetRear%20Light _returnvalue_3))
    (:then_3
      ;[0.08653 0.329 1] Create material instance for light on mesh and save it as a variable
      (if (not (== (Utilities|Array|FindItem (Class|MeshComponent|GetMaterialSlotNames (Variables|Default|GetCar%20Body%20mesh)) "Lights") -1))
        (bind _returnvalue_4 (Rendering|Material|CreateDynamicMaterialInstance (Variables|Default|GetCar%20Body%20mesh) (Utilities|Array|FindItem (Class|MeshComponent|GetMaterialSlotNames (Variables|Default|GetCar%20Body%20mesh)) "Lights") (Rendering|Material|GetMaterial (Variables|Default|GetCar%20Body%20mesh) (Utilities|Array|FindItem (Class|MeshComponent|GetMaterialSlotNames (Variables|Default|GetCar%20Body%20mesh)) "Lights")) "None" :!class /Script/Engine.PrimitiveComponent))
        (Variables|System|SetLights%20material%20instance _returnvalue_4)
        (Rendering|Material|SetVectorParameterValue _returnvalue_4 "Front Lights Color" (Variables|Lights|GetFront%20light%20color) :!class /Script/Engine.MaterialInstanceDynamic)
        (Rendering|Material|SetScalarParameterValue _returnvalue_4 "Random per instance" (Math|Random|RandomFloatinRange 0.0 1.0) :!class /Script/Engine.MaterialInstanceDynamic)))
    (:then_4
      ;[0.9019 0.377 1] Set car color
      (if (not (== (Utilities|Array|FindItem (Class|MeshComponent|GetMaterialSlotNames (Variables|Default|GetCar%20Body%20mesh)) "Body") -1))
        (bind _returnvalue_5 (Rendering|Material|CreateDynamicMaterialInstance (Variables|Default|GetCar%20Body%20mesh) (Utilities|Array|FindItem (Class|MeshComponent|GetMaterialSlotNames (Variables|Default|GetCar%20Body%20mesh)) "Body") (Rendering|Material|GetMaterial (Variables|Default|GetCar%20Body%20mesh) (Utilities|Array|FindItem (Class|MeshComponent|GetMaterialSlotNames (Variables|Default|GetCar%20Body%20mesh)) "Body")) "None" :!class /Script/Engine.PrimitiveComponent))
        (bind _output_get (Variables|System|SetBody%20Material%20Instance _returnvalue_5))
        (Rendering|Material|SetVectorParameterValue _output_get "Color" (Utilities|Array|Get(acopy) _car_colors (select (Variables|Color|GetSpecific%20color?) _returnvalue (Math|Random|RandomIntegerinRange 0 _returnvalue))) :!class /Script/Engine.MaterialInstanceDynamic)
        (CallFunction|SetDirtiness (Variables|Dirtiness|GetDirtiness%20color) 0.0 true)))))

(event Custom|Enable%20indicator
  (params (Indicator%20type :type Enum_TurnType%20Enum :default "NewEnumerator0") (Hazard? :type Boolean) (Temporary? :type Boolean))
  ;[1 0.4466 0.183] Toggle indicator
  (Variables|Default|SetTemporary%20indicator Temporary?)
  (Variables|System|SetIndicator%20state Indicator%20type)
  (Variables|Lights|SetHazard? Hazard?) ; Added in 1.1 update
  (bind _lights_material_instance (Variables|System|GetLights%20material%20instance)
    (:then
      (Rendering|Material|SetScalarParameterValue _lights_material_instance "Right indicator on" (select (Variables|Lights|GetHazard?) 1.0 (Utilities|Select :Index Indicator%20type :NewEnumerator0 0.0 :NewEnumerator1 1.0 :NewEnumerator2 0.0)) :!class /Script/Engine.MaterialInstanceDynamic)
      (Rendering|Material|SetScalarParameterValue (Variables|System|GetLights%20material%20instance) "Left indicator on" (select (Variables|Lights|GetHazard?) 1.0 (Utilities|Select :Index Indicator%20type :NewEnumerator0 0.0 :NewEnumerator1 0.0 :NewEnumerator2 1.0)) :!class /Script/Engine.MaterialInstanceDynamic))
    (:else)))

(event Custom|Enable%20headlights
  (params (Enable? :type Boolean))
  ;[0.4463 1 0.9602] Toggle headlights
  (Variables|System|SetHeadlights%20on? Enable?)
  (bind _lights_material_instance (Variables|System|GetLights%20material%20instance)
    (:then
      (Rendering|Material|SetScalarParameterValue _lights_material_instance "Front Lights on" (Math|Conversions|ToFloat(Boolean) Enable?) :!class /Script/Engine.MaterialInstanceDynamic))
    (:else
      _))
  (Rendering|Components|Light|SetIntensity (Variables|Default|GetFront%20light) (select (Variables|System|GetHeadlights%20on?) (Variables|Lights|GetFront%20Light%20intensity) 0.0))
  (Rendering|Components|Light|SetIntensity (Variables|Default|GetRear%20Light) (select (Variables|System|GetHeadlights%20on?) (Variables|Lights|GetRear%20light%20intencity) 0.0)))

(event Custom|Brake%20light
  (params (Enable? :type Boolean))
  ;[0.3073 1 0.3073] Toggle Brake lights
  (Variables|System|SetBrake%20light%20enabled? Enable?)
  (bind _lights_material_instance (Variables|System|GetLights%20material%20instance)
    (:then
      (Rendering|Material|SetScalarParameterValue _lights_material_instance "Brake light on" (Math|Conversions|ToFloat(Boolean) Enable?) :!class /Script/Engine.MaterialInstanceDynamic))
    (:else
      _))
  (Rendering|Components|Light|SetIntensity (Variables|Default|GetRear%20Light) (select Enable? (* (Variables|Lights|GetRear%20light%20intencity) 3.0) (select (Variables|System|GetHeadlights%20on?) (Variables|Lights|GetRear%20light%20intencity) 0.0))))

(event Custom|Enable%20Reverse%20Light
  (params (Enabled? :type Boolean))
  ;[1 1 1] Reverse Light
  (bind _lights_material_instance (Variables|System|GetLights%20material%20instance)
    (:then
      (Rendering|Material|SetScalarParameterValue _lights_material_instance "Reverse light on" (Math|Conversions|ToFloat(Boolean) Enabled?) :!class /Script/Engine.MaterialInstanceDynamic))
    (:else)))

(event EventBeginPlay
  (bind _returnvalue (Components|GetOwner))
  (bind _asmesh_component (Utilities|Casting|CastToMeshComponent (Variables|/Script/Engine.Actor|GetRootComponent _returnvalue))
    (:then
      (CallFunction|SetUpCarBody _returnvalue _asmesh_component))
    (:CastFailed
      (Development|PrintString "Traffic AI System error: Root component of your vehicle is not a mesh" true true "(R=1.000000,G=0.000000,B=0.007126,A=1.000000)" 5.0))))

(fn OpenDoor
  (params (Door :type Enum_Car_doors%20Enum :default "NewEnumerator0") (Open? :type Boolean))
  (LocalVariables|SetDoor%20to%20open Door)
  (LocalVariables|SetOpen?%20Local Open?)
  (Utilities|FlowControl|Sequence
    (:then_0
      (Utilities|FlowControl|DoOnce false
        (:Completed
          (bind _asskeletal_mesh_component (Utilities|Casting|CastToSkeletalMeshComponent (Variables|Default|GetCar%20Body%20mesh))
            (:then
              (bind _asabp_traffic_car (Utilities|Casting|CastToABP_Traffic_Car (Components|SkeletalMesh|GetAnimInstance _asskeletal_mesh_component))
                (:then
                  (bind _output_get (LocalVariables|SetAnim%20Instance _asabp_traffic_car))
                  (Variables|/Game/Traffic_AI_System/Cars/ABP_Traffic_Car.ABP_Traffic_Car_C|SetFront%20doors _output_get (Variables|Openabledoors|GetFront%20doors%20opened))
                  (Variables|/Game/Traffic_AI_System/Cars/ABP_Traffic_Car.ABP_Traffic_Car_C|SetRear%20doors _output_get (Variables|Openabledoors|GetRear%20doors%20opened)))
                (:CastFailed
                  (Development|PrintString "Traffic AI System Warning: Vehicle Anim Instance is not \"ABP_Traffic_Car\", doors can't be opened." true true "(R=1.000000,G=0.350113,B=0.000000,A=1.000000)" 7.0))))
            (:CastFailed
              (Development|PrintString "Traffic AI System Warning: Attempted to use \"Open door\" function in Apperance component, but vehicle mesh is not Skeletal Mesh" true true "(R=1.000000,G=0.350113,B=0.000000,A=1.000000)" 7.0))))))
    (:then_1
      (Utilities|Map|Add (Variables|/Game/Traffic_AI_System/Cars/ABP_Traffic_Car.ABP_Traffic_Car_C|GetDoors%20state (LocalVariables|GetAnim%20Instance)) (LocalVariables|GetDoor%20to%20open) (LocalVariables|GetOpen?%20Local)))
    (:then_2
      (return))))

(fn SetDirtiness
  (params (Dirtiness%20color :type Linear%20Color%20Structure) (Dirtiness%20%280%20-%201%29 :type Float%20%28single-precision%29) (Random%20dirtiness :type Boolean))
  (Utilities|FlowControl|Sequence
    (:then_0
      (Rendering|Material|SetVectorParameterValue (Variables|System|GetBody%20Material%20Instance) "Dirtiness color" Dirtiness%20color :!class /Script/Engine.MaterialInstanceDynamic)
      (if Random%20dirtiness
        (if (Math|Random|RandomBoolwithWeight (Variables|Dirtiness|GetChance%20for%20dirty%20car))
          (bind _output_get (Variables|Dirtiness|SetDirtiness (* (Math|Float|Power (Math|Random|RandomFloatinRange 0.0 1.0) (Variables|Dirtiness|GetDirtiness%20chance%20%28power%29)) (Variables|Dirtiness|GetDirtness%20multiplier))))
          (Rendering|Material|SetScalarParameterValue (Variables|System|GetBody%20Material%20Instance) "Dirtiness" _output_get :!class /Script/Engine.MaterialInstanceDynamic)
          (else
            (Rendering|Material|SetScalarParameterValue (Variables|System|GetBody%20Material%20Instance) "Dirtiness" 0.0 :!class /Script/Engine.MaterialInstanceDynamic)
            (Variables|Dirtiness|SetDirtiness 0.0)))
        (else
          (bind _output_get_2 (Variables|Dirtiness|SetDirtiness Dirtiness%20%280%20-%201%29))
          (Rendering|Material|SetScalarParameterValue (Variables|System|GetBody%20Material%20Instance) "Dirtiness" _output_get_2 :!class /Script/Engine.MaterialInstanceDynamic))))
    (:then_1
      (return))))