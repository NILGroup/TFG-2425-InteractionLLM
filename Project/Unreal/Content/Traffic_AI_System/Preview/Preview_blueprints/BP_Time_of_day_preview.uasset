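; Preview time-of-day controller for the traffic AI system that drives a directional light as the sun.
; Each Tick advances TimeOfDay by a scaled TimePlayRate per frame, wraps past 24 hours and maps it to sun pitch.
; It pushes the time to a main road reference, found by scanning traffic path actors whenever that reference is invalid.
; The construction script applies the same sun rotation in the editor.
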(event EventTick
  (params (DeltaSeconds :type Float%20%28single-precision%29))
  ;[0.3073 1 0.3073] If main road is not valid - find it
  (Utilities|IsValid (Variables|Default|GetMain%20Road%20Time%20of%20Day)
    (:Is%20Valid
      ;[1 0.8555 0.2249] Set time of day
      (Variables|Default|SetTime%20of%20day (select (> (+ (Variables|Default|GetTime%20of%20day) (* (Variables|Default|GetTime%20play%20rate) 0.0001)) 24.0) 0.0 (+ (Variables|Default|GetTime%20of%20day) (* (Variables|Default|GetTime%20play%20rate) 0.0001))))
      ;[0.9787 0.6273 1] Set Sun rotation
      (Transformation|SetWorldRotation (Variables|/Script/Engine.Light|GetLightComponent (Variables|Default|GetDirectional%20light)) (Math|Rotator|MakeRotator 0.0 (+ (Math|Float|MapRangeClamped (Variables|Default|GetTime%20of%20day) 0.0 24.0 0.0 3.6e+02) 9e+01) 45.0) false false)
      ;[1 0.1042 0.1042] Set Time of day in Main Road
      (Variables|/Game/Traffic_AI_System/Blueprints/BP_Traffic_path_50_Parent.BP_Traffic_path_50_Parent_C|SetTime%20of%20day (Variables|Default|GetMain%20Road%20Time%20of%20Day) (Variables|Default|GetTime%20of%20day)))
    (:Is%20Not%20Valid
      ;[0.4463 1 0.9602] Find Main Road
      (bind _outactors (Actor|GetAllActorsOfClass "/Game/Traffic_AI_System/Blueprints/BP_Traffic_path_50_Parent.BP_Traffic_path_50_Parent_C"))
      (for _array_element _outactors
        (Variables|Default|SetMain%20Road%20Time%20of%20Day (Variables|/Game/Traffic_AI_System/Blueprints/BP_Traffic_path_50_Parent.BP_Traffic_path_50_Parent_C|GetMain%20Road _array_element))))))

(fn ConstructionScript
  (Transformation|SetWorldRotation (Variables|/Script/Engine.Light|GetLightComponent (Variables|Default|GetDirectional%20light)) (Math|Rotator|MakeRotator 0.0 (+ (Math|Float|MapRangeClamped (Variables|Default|GetTime%20of%20day) 0.0 24.0 0.0 3.6e+02) 9e+01) 45.0) false false))