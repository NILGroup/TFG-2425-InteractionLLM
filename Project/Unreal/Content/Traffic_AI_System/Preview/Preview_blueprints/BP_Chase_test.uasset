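; Preview trigger actor that starts a car chase in the Traffic AI System, firing once when BP_Preview_pawn overlaps it.
; If Target is valid, each valid car in BlackCars navigates toward it, excluding it from sphere traces.
; Target switches to roam mode with despawn checks off.
; Pursuers and Target all speed through traffic lights with a single accident behaviour, set through their BP_Traffic_Car_Component.
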(event Collision|EventActorBeginOverlap
  (params (OtherActor :type Actor%20Object%20Reference))
  (bind _target (Variables|Default|GetTarget))
  (bind _returnvalue (Actor|GetComponentbyClass _target "/Game/Traffic_AI_System/Components/BP_Traffic_Car_Component.BP_Traffic_Car_Component_C"))
  (Utilities|Casting|CastToBP_Preview_pawn OtherActor)
  (Utilities|FlowControl|DoOnce false
    (:Completed
      (Utilities|IsValid (Variables|Default|GetTarget)
        (:Is%20Valid
          (for _array_element (Variables|Default|GetBlack%20cars)
            (Utilities|IsValid _array_element
              (:Is%20Valid
                (Default|SetAIModetoNavigatetoPoint (Actor|GetComponentbyClass _array_element "/Game/Traffic_AI_System/Components/BP_Traffic_Car_Component.BP_Traffic_Car_Component_C") (Variables|Default|GetTarget) "0, 0, 0" 0 false "NewEnumerator4" 2.5e+02 false true)
                (Default|SetSpeeding (Actor|GetComponentbyClass _array_element "/Game/Traffic_AI_System/Components/BP_Traffic_Car_Component.BP_Traffic_Car_Component_C") true true)
                (Variables|/Game/Traffic_AI_System/Components/BP_Traffic_Car_Component.BP_Traffic_Car_Component_C|SetAccident%20behaviours (Actor|GetComponentbyClass _array_element "/Game/Traffic_AI_System/Components/BP_Traffic_Car_Component.BP_Traffic_Car_Component_C") (Utilities|Array|MakeArray "NewEnumerator0")))))
          (Default|SetAIModetoRoam _returnvalue 0 false)
          (Default|SetSpeeding _returnvalue true true)
          (Default|SetCheckforDespawn _returnvalue false)
          (Variables|/Game/Traffic_AI_System/Components/BP_Traffic_Car_Component.BP_Traffic_Car_Component_C|SetAccident%20behaviours _returnvalue (Utilities|Array|MakeArray "NewEnumerator0")))))))

(fn ConstructionScript)