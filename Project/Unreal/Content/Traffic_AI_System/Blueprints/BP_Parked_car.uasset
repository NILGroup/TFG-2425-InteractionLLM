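; Placeable parking spot for the traffic AI that spawns a random parked car near the player or camera.
; A distance-scaled timer checks range and a shared count on one main instance, optionally requiring off-screen or trace-occluded locations after initial setup.
; It finds the nearest traffic path, can register there as parking, and can send its car into traffic when clear.
; Construction optionally snaps it to surfaces and color-codes the debug mesh.
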(event Custom|Initialize%20Start%20Driving
  (bind _assigned_car (Variables|System|GetAssigned%20car))
  (bind _nearest_road (Variables|System|GetNearest%20Road))
  (bind _returnvalue (Actor|GetComponentbyClass _assigned_car "/Game/Traffic_AI_System/Components/BP_Traffic_Car_Component.BP_Traffic_Car_Component_C"))
  ;[0.2282 0.5915 1] Start driving
  (if (Variables|Basic|GetCan%20start%20driving?)
    (Utilities|FlowControl|RetriggerableDelay (Math|Random|RandomFloatinRange 1e+01 (Math|Float|Clamp(Float) (Variables|Advanced|GetStart%20driving%20max%20delay) 11.0 65536.0)))
    (Utilities|IsValid (Variables|System|GetAssigned%20car)
      (:Is%20Valid
        ;;[1 0.269 0.6684] Check if there are no cars on the road
        (bind _too_close_to_other_cars_ (Default|CheckifTooClosetoSplineLengths _nearest_road (Variables|/Game/Traffic_AI_System/Blueprints/BP_Traffic_path_50_Parent.BP_Traffic_path_50_Parent_C|GetActors%20sorted%20float _nearest_road) (Default|FindSplineDistanceClosesttoLocation (Variables|System|GetNearest%20Road) (Transformation|GetActorLocation (Variables|System|GetAssigned%20car)))))
        (if _too_close_to_other_cars_
          (CallFunction|TrytoJoinTraffic 5.0)
          (else
            (switch Utilities|FlowControl|Switch|SwitchonEnum_Car_mode (Variables|/Game/Traffic_AI_System/Components/BP_Traffic_Car_Component.BP_Traffic_Car_Component_C|GetCar%20mode _returnvalue) ; Only start driving if mode is set to Park
              (:NewEnumerator1
                (Variables|/Game/Traffic_AI_System/Components/BP_Traffic_Car_Component.BP_Traffic_Car_Component_C|SetUpdate%20index _returnvalue (+ (Variables|/Game/Traffic_AI_System/Components/BP_Traffic_Car_Component.BP_Traffic_Car_Component_C|GetInitial%20adjust%20max%20index _returnvalue) 1))
                ;;[0.3844 1 0.7542] Add one to the Number of AI Cars, and subtract 1 from Number of Parked Cars
                (Default|AddCar (Variables|/Game/Traffic_AI_System/Blueprints/BP_Traffic_path_50_Parent.BP_Traffic_path_50_Parent_C|GetMain%20Road (Variables|System|GetRoad)) 1)
                (CallFunction|AddParkedCar (Variables|System|GetMain%20Parked%20Car) -1)
                (Default|InitializeVehicle _returnvalue (Variables|System|GetNearest%20Road) (Variables|System|GetAssigned%20car))
                (Utilities|FlowControl|Delay 0.2)
                (Default|DisableParking _returnvalue 6e+01 false)))))))))

(event Custom|Try%20to%20join%20traffic
  (params (Delay :type Float%20%28double-precision%29))
  (bind _assigned_car (Variables|System|GetAssigned%20car))
  (bind _nearest_road (Variables|System|GetNearest%20Road))
  (bind _returnvalue (Actor|GetComponentbyClass _assigned_car "/Game/Traffic_AI_System/Components/BP_Traffic_Car_Component.BP_Traffic_Car_Component_C"))
  (Utilities|FlowControl|RetriggerableDelay Delay)
  ;[0.2282 0.5915 1] Start driving
  (Utilities|IsValid (Variables|System|GetAssigned%20car)
    (:Is%20Valid
      ;;[1 0.269 0.6684] Check if there are no cars on the road
      (bind _too_close_to_other_cars_ (Default|CheckifTooClosetoSplineLengths _nearest_road (Variables|/Game/Traffic_AI_System/Blueprints/BP_Traffic_path_50_Parent.BP_Traffic_path_50_Parent_C|GetActors%20sorted%20float _nearest_road) (Default|FindSplineDistanceClosesttoLocation (Variables|System|GetNearest%20Road) (Transformation|GetActorLocation (Variables|System|GetAssigned%20car)))))
      (if _too_close_to_other_cars_
        (CallFunction|TrytoJoinTraffic 5.0)
        (else
          (switch Utilities|FlowControl|Switch|SwitchonEnum_Car_mode (Variables|/Game/Traffic_AI_System/Components/BP_Traffic_Car_Component.BP_Traffic_Car_Component_C|GetCar%20mode _returnvalue) ; Only start driving if mode is set to Park
            (:NewEnumerator1
              (Variables|/Game/Traffic_AI_System/Components/BP_Traffic_Car_Component.BP_Traffic_Car_Component_C|SetUpdate%20index _returnvalue (+ (Variables|/Game/Traffic_AI_System/Components/BP_Traffic_Car_Component.BP_Traffic_Car_Component_C|GetInitial%20adjust%20max%20index _returnvalue) 1))
              ;;[0.3844 1 0.7542] Add one to the Number of AI Cars, and subtract 1 from Number of Parked Cars
              (Default|AddCar (Variables|/Game/Traffic_AI_System/Blueprints/BP_Traffic_path_50_Parent.BP_Traffic_path_50_Parent_C|GetMain%20Road (Variables|System|GetRoad)) 1)
              (CallFunction|AddParkedCar (Variables|System|GetMain%20Parked%20Car) -1)
              (Default|InitializeVehicle _returnvalue (Variables|System|GetNearest%20Road) (Variables|System|GetAssigned%20car))
              (Utilities|FlowControl|Delay 0.2)
              (Default|DisableParking _returnvalue 6e+01 false))))))))

(event Custom|Parked%20Car%20Timer
  (bind _returnvalue (Game|GetPlayerController 0))
  (bind _returnvalue_2 (Viewport|GetViewportSize))
  (bind _staticmesh (Variables|Default|GetStaticMesh))
  (bind _road_type (Variables|Basic|GetRoad%20Type))
  (bind _road (Variables|System|GetRoad))
  (bind _staticmesh_2 (Variables|Default|GetStaticMesh))
  (bind _returnvalue_3 (Transformation|GetWorldLocation _staticmesh))
  (bind _returnvalue_4 (Transformation|GetWorldTransform _staticmesh_2))
  (bind _spawn_cars (Variables|/Game/Traffic_AI_System/Blueprints/BP_Traffic_path_50_Parent.BP_Traffic_path_50_Parent_C|GetSpawn%20Cars _road))
  (bind _value (Utilities|Map|Find _spawn_cars _road_type))
  (bind _screenposition (Class|GameplayStatics|ProjectWorldtoScreen _returnvalue _returnvalue_3 false))
  ;[0.2577 1 0.2174] Random delay prevents cars from spawning in order at which you was placing Parked Car actors.
  (Utilities|FlowControl|Delay (select (Variables|System|GetInitial%20setup) (Math|Random|RandomFloatinRange 0.0 2.0) 0.0))
  ;[0.3844 1 0.7542] Check if can spawn more vehicles
  (if (not (>= (Variables|BP_Parked_car_C|GetNumber%20of%20parked%20cars (Variables|System|GetMain%20Parked%20Car)) (Variables|Settings|GetMax%20Parked%20Cars)))
    ;[1 0.7097 0.2625] Get Spawn Center Location (a location around which the traffic will spawn), usually it is the location of the player or camera
    (bind _output_get (Variables|System|SetSpawn%20center%20location (Utilities|Select :Index (Variables|Settings|GetTraffic%20center%20location%20type) :NewEnumerator0 (Transformation|GetWorldLocation (Variables|/Script/Engine.PlayerCameraManager|GetTransformComponent (Game|GetPlayerCameraManager 0))) :NewEnumerator1 (Transformation|GetActorLocation (Game|Player|GetPlayerPawn 0)) :NewEnumerator2 (CallFunction|GetTrafficSpawnCenterLocation) :NewEnumerator3 "0, 0, 0")))
    ;[1 0.269 0.6684] Check if spawn location is in spawn distance range. If initial setup, ignore MIN value.
    (bind _output_get_2 (Variables|System|SetDistance%20to%20player (Math|Vector|Distance(Vector) _output_get (Transformation|GetWorldLocation (Variables|Default|GetStaticMesh)))))
    (if (Math|Float|InRange(Float) _output_get_2 (select (Variables|System|GetInitial%20setup) 0.0 (Variables|Settings|GetSpawn%20distance%20min)) (Variables|Settings|GetSpawn%20distance%20max))
      ;[0.2577 1 0.2174] Set timer based on the distance to player. This saves performance.
      (CallFunction|ResetTimer (Math|Float|MapRangeClamped _output_get_2 2e+03 7.5e+04 0.5 7.0))
      ;[1 0.4454 0.295] If this setting is set to TRUE, cars will try to spawn only off screen or behind objects. If set to FALSE, cars will spawn even in front of the player. Spawning behind objects is based on one simple line trace, so sometimes you may see that the car spawned.
      (if (Variables|Settings|GetSpawn%20only%20off%20screen)
        ;[0.2577 1 0.2174] If initial setup, spawn cars no matter if they are visible by player or not.
        (if (Variables|System|GetInitial%20setup)
          (Utilities|IsValid (Variables|System|GetAssigned%20car) :!label _label
            (:Is%20Valid
              ;[0.151 0.151 0.151] Set Initial Setup to false when initial setup is done
              (Variables|System|SetInitial%20setup false))
            (:Is%20Not%20Valid
              (Variables|System|SetInitial%20setup false)
              ;[0.7124 0.3851 1] Select random car and spawn it
              (bind _keys (Utilities|Map|Keys (.vehicle _value)))
              (bind _output_get_3 (Variables|System|SetCar%20to%20spawn (Utilities|Array|Get(acopy) _keys (Math|Random|RandomIntegerinRange 0 (Utilities|Array|LastIndex _keys)))))
              (if (Math|Random|RandomBoolwithWeight (.Value (Utilities|Map|Find (.vehicle _value) _output_get_3)))
                (bind _returnvalue_5 (Game|SpawnActorfromClass (Variables|System|GetCar%20to%20spawn) (Math|Transform|MakeTransform (+ (.location _returnvalue_4) (Math|Vector|MakeVector 0.0 0.0 (Variables|Advanced|GetSpawn%20Z%20offset))) (.rotation _returnvalue_4) "1.000000,1.000000,1.000000") "AdjustIfPossibleButDontSpawnIfColliding" 0 0))
                (Utilities|IsValid _returnvalue_5
                  (:Is%20Valid
                    (Transformation|AddWorldOffset (Actor|GetComponentbyClass _returnvalue_5 "/Script/Engine.SkeletalMeshComponent") (Math|Vector|MakeVector 0.0 0.0 (* (Variables|Advanced|GetSpawn%20Z%20offset) -1.0)) false true)
                    ;[1 0.2592 0.6005] Check if vehicle was spawned correctly, and initialize it
                    (Utilities|Time|PauseTimerbyHandle (Variables|System|GetSpawn%20Timer))
                    (Variables|/Game/Traffic_AI_System/Components/BP_Traffic_Car_Component.BP_Traffic_Car_Component_C|SetSelected%20parking%20spot (Actor|GetComponentbyClass _returnvalue_5 "/Game/Traffic_AI_System/Components/BP_Traffic_Car_Component.BP_Traffic_Car_Component_C") self)
                    (bind _output_get_4 (Variables|System|SetAssigned%20car _returnvalue_5))
                    (Default|InitializeVehicle (Actor|GetComponentbyClass _returnvalue_5 "/Game/Traffic_AI_System/Components/BP_Traffic_Car_Component.BP_Traffic_Car_Component_C") 0 _output_get_4)
                    (CallFunction|InitializeStartDriving))))))
          (else
            ;[1 0.7097 0.2625] Check for objects between car spawn location and player
            (bind _hidden_ (CallFunction|VisibilityCheckParkedCar (Variables|Default|GetCar%20spawn%20visibility%20iterations)))
            ;[0.2577 1 0.2174] If spawn location is off screen OR behind something, the car will spawn
            (if (or _hidden_ (not (Math|Boolean|ANDBoolean (> (.x _screenposition) 0.0) (> (.y _screenposition) 0.0) (< (.x _screenposition) (.x _returnvalue_2)) (< (.y _screenposition) (.y _returnvalue_2)))))
              (goto _label))))
        (else
          (goto _label)))
      (else
        (Variables|System|SetInitial%20setup false)
        (CallFunction|ResetTimer (Math|Float|MapRangeClamped _output_get_2 2e+03 7.5e+04 0.5 7.0))))))

(event Custom|Reset%20timer
  (params (Time :type Float%20%28double-precision%29))
  ;[1 0.7097 0.2625] Run Parked Car Timer for the first time, and then start the timer
  (Utilities|Time|UnpauseTimerbyHandle (Variables|System|GetSpawn%20Timer))
  (bind _returnvalue (Utilities|Time|SetTimerbyEvent (delegate Custom|Parked%20Car%20Timer) (* (Math|Float|Clamp(Float) Time 1.0 6e+01) (Math|Random|RandomFloatinRange 0.9 1.1)) true))
  (Variables|System|SetSpawn%20Timer _returnvalue))

(event EventBeginPlay
  (Utilities|FlowControl|Sequence
    (:then_0
      ;[0.4463 1 0.9602] Set Main Parked Car
      (Utilities|IsValid (Variables|System|GetMain%20Parked%20Car)
        (:Is%20Not%20Valid
          (bind _outactors (Actor|GetAllActorsOfClass "BP_Parked_car_C"))
          (for _array_element _outactors
            (Variables|BP_Parked_car_C|SetMain%20Parked%20Car _array_element self))
          (bind _outactors_2 (Actor|GetAllActorsOfClass "/Game/Traffic_AI_System/Blueprints/BP_Traffic_path_50_Parent.BP_Traffic_path_50_Parent_C"))
          (for _array_element_2 _outactors_2
            (Variables|/Game/Traffic_AI_System/Blueprints/BP_Traffic_path_50_Parent.BP_Traffic_path_50_Parent_C|SetMain%20Parked%20Car _array_element_2 (Variables|System|GetMain%20Parked%20Car))))))
    (:then_1
      (CallFunction|FindNearestRoad))
    (:then_2
      ;[1 0.05203 0.06197] Get random Traffic Path to get Spawn Cars map
      (bind _returnvalue (Actor|GetActorOfClass "/Game/Traffic_AI_System/Blueprints/BP_Traffic_path_50_Parent.BP_Traffic_path_50_Parent_C"))
      (Variables|System|SetRoad _returnvalue))
    (:then_3
      ;[0.3139 0.6562 1] Add to Parking Spots
      (if (Variables|Basic|GetCan%20park%20here?)
        (Utilities|Array|AddUnique (Variables|/Game/Traffic_AI_System/Blueprints/BP_Traffic_path_50_Parent.BP_Traffic_path_50_Parent_C|GetParking%20Spots (Variables|System|GetNearest%20Road)) self)))
    (:then_4
      ;[0.2577 1 0.2174] Chance to spawn a car. If false, car will not be spawned in this location.
      (if (Math|Random|RandomBoolwithWeight (Variables|Basic|GetChance%20to%20spawn%20a%20car%20here))
        ;[1 0.7097 0.2625] Run Parked Car Timer for the first time, and then start the timer
        (CallFunction|ParkedCarTimer)
        (bind _returnvalue_2 (Utilities|Time|SetTimerbyEvent (delegate Custom|Parked%20Car%20Timer) (* (Math|Float|Clamp(Float) (stale Custom|Reset%20timer Time) 1.0 6e+01) (Math|Random|RandomFloatinRange 0.9 1.1)) true))
        (Variables|System|SetSpawn%20Timer _returnvalue_2)))))

(fn ConstructionScript
  (bind _can_start_driving_ (Variables|Basic|GetCan%20start%20driving?))
  (bind _can_park_here_ (Variables|Basic|GetCan%20park%20here?))
  (bind _returnvalue (select _can_park_here_ "(R=1.000000,G=0.116427,B=0.000000,A=1.000000)" "(R=0.000000,G=1.000000,B=0.000000,A=1.000000)"))
  (bind _returnvalue_2 (select _can_start_driving_ "(R=0.000000,G=0.000000,B=1.000000,A=1.000000)" _returnvalue))
  (Utilities|FlowControl|Sequence
    (:then_0
      ;[1 0.8555 0.2249] Align to surface
      (if (Variables|Basic|GetAlign%20to%20surface)
        (bind (_outhit _returnvalue_3) (Collision|LineTraceForObjects (+ (Transformation|GetWorldLocation (Variables|Default|GetStaticMesh)) "0, 0,200.000000") (+ (Transformation|GetWorldLocation (Variables|Default|GetStaticMesh)) "0.000000,0.000000,-200.000000") (Variables|Advanced|GetStick%20to%20object%20types) false 0 "None"))
        (if _returnvalue_3
          (Transformation|SetWorldLocationAndRotation (Variables|Default|GetStaticMesh) (.Location (Collision|BreakHitResult _outhit)) (Math|Rotator|MakeRotator (.Roll (Math|Rotator|BreakRotator (Math|Rotator|MakeRotationfromAxes (Math|Vector|CrossProduct (Math|Vector|GetRightVector (Variables|Default|GetStaticMesh)) (.ImpactNormal (Collision|BreakHitResult _outhit))) (Math|Vector|CrossProduct (.ImpactNormal (Collision|BreakHitResult _outhit)) (Math|Vector|CrossProduct (Math|Vector|GetRightVector (Variables|Default|GetStaticMesh)) (.ImpactNormal (Collision|BreakHitResult _outhit)))) (.ImpactNormal (Collision|BreakHitResult _outhit))))) (.Pitch (Math|Rotator|BreakRotator (Math|Rotator|MakeRotationfromAxes (Math|Vector|CrossProduct (Math|Vector|GetRightVector (Variables|Default|GetStaticMesh)) (.ImpactNormal (Collision|BreakHitResult _outhit))) (Math|Vector|CrossProduct (.ImpactNormal (Collision|BreakHitResult _outhit)) (Math|Vector|CrossProduct (Math|Vector|GetRightVector (Variables|Default|GetStaticMesh)) (.ImpactNormal (Collision|BreakHitResult _outhit)))) (.ImpactNormal (Collision|BreakHitResult _outhit))))) (.yaw (Transformation|GetWorldRotation (Variables|Default|GetStaticMesh)))) false false))))
    (:then_1
      ;[0.3073 1 0.3073] Set debug mesh color
      (bind _returnvalue_4 (Rendering|Material|CreateDynamicMaterialInstance (Variables|Default|GetStaticMesh) 0 "/Game/Traffic_AI_System/Misc/Materials/M_Parked_car_debug_material.M_Parked_car_debug_material" "None" :!class /Script/Engine.PrimitiveComponent))
      (Rendering|Material|SetVectorParameterValue _returnvalue_4 "Color" _returnvalue_2 :!class /Script/Engine.MaterialInstanceDynamic)
      (Rendering|Material|SetVectorParameterValue _returnvalue_4 "Secondary Color" (select (Variables|Basic|GetCan%20park%20here?) "(R=1.000000,G=0.116427,B=0.000000,A=1.000000)" _returnvalue_2) :!class /Script/Engine.MaterialInstanceDynamic)
      (Rendering|Material|SetScalarParameterValue _returnvalue_4 "Opacity" (Variables|Basic|GetChance%20to%20spawn%20a%20car%20here) :!class /Script/Engine.MaterialInstanceDynamic))))

(fn GetTrafficSpawnCenterLocation
  (return (Camera|GetCameraLocation (Game|GetPlayerCameraManager 0))))

(fn AddParkedCar
  (params (Ammount%20to%20add :type Integer))
  (Variables|BP_Parked_car_C|SetNumber%20of%20parked%20cars (Variables|System|GetMain%20Parked%20Car) (+ (Variables|BP_Parked_car_C|GetNumber%20of%20parked%20cars (Variables|System|GetMain%20Parked%20Car)) Ammount%20to%20add))
  (return))

(fn VisibilityCheckParkedCar
  (params (Iterations :type Integer))
  (for _index (range 0 Iterations)
    (bind _returnvalue (Collision|LineTraceByChannel (+ (.Origin (Collision|GetComponentBounds (Variables|Default|GetStaticMesh))) (* (Utilities|Select :Index _index :Option%200 "0, 0,0.500000" :Option%201 "1.000000,0.000000,0.250000" :Option%202 "-1.000000,0.000000,0.250000" :Option%203 "0.000000,-0.500000,0.250000" :Option%204 "0.000000,0.500000,0.250000" :Option%205 (Math|Vector|MakeVector (Math|Random|RandomFloatinRange -1.0 1.0) (Math|Random|RandomFloatinRange -0.5 0.5) (Math|Random|RandomFloatinRange 0.0 0.5))) (.SphereRadius (Collision|GetComponentBounds (Variables|Default|GetStaticMesh))))) (Variables|System|GetSpawn%20center%20location) "TraceTypeQuery1" false 0 "None" true "(R=1.000000,G=0.000000,B=0.000000,A=1.000000)" "(R=0.000000,G=1.000000,B=0.000000,A=1.000000)" 1.0))
    (if (not _returnvalue)
      (return false)))
  (return true))

(fn FindNearestRoad
  ;[0.236 0.6706 1] Find nearest road
  (Variables|System|SetDistance%20to%20nearest%20road 1e+07)
  (bind _outactors (Actor|GetAllActorsOfClass "/Game/Traffic_AI_System/Blueprints/BP_Traffic_path_50_Parent.BP_Traffic_path_50_Parent_C"))
  (for _array_element _outactors
    (if (< (Math|Vector|Distance(Vector) (Spline|GetLocationatDistanceAlongSpline (Variables|/Game/Traffic_AI_System/Blueprints/BP_Traffic_path_50_Parent.BP_Traffic_path_50_Parent_C|GetSecond%20spline _array_element) (Default|FindSplineDistanceClosesttoLocation _array_element (Transformation|GetWorldLocation (Variables|Default|GetStaticMesh))) "World") (Transformation|GetWorldLocation (Variables|Default|GetStaticMesh))) (Variables|System|GetDistance%20to%20nearest%20road))
      (Variables|System|SetDistance%20to%20nearest%20road (Math|Vector|Distance(Vector) (Spline|GetLocationatDistanceAlongSpline (Variables|/Game/Traffic_AI_System/Blueprints/BP_Traffic_path_50_Parent.BP_Traffic_path_50_Parent_C|GetSecond%20spline _array_element) (Default|FindSplineDistanceClosesttoLocation _array_element (Transformation|GetWorldLocation (Variables|Default|GetStaticMesh))) "World") (Transformation|GetWorldLocation (Variables|Default|GetStaticMesh))))
      (Variables|System|SetNearest%20Road _array_element)))
  (return))