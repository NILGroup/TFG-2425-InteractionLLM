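; Experiment setup manager that picks the participant user ID and group for the next experiment session.
; On BeginPlay it loads group ID lists and last-experiment data from data tables, then opens the setup panel widget in UI-only input mode.
; GetNextUser either stays in the current group or alternates through wrapped group enum values, tracking a clamped index per group.
; ResetNextUser restores the selection to the last experiment's data.
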(event Custom|InitExperimentSetUpPanel
  (bind _returnvalue (Game|GetPlayerController 0))
  (Input|SetInputModeUIOnly _returnvalue 0 "DoNotLock" false)
  (Variables|/Script/Engine.PlayerController|SetbShowMouseCursor _returnvalue true)
  (bind _returnvalue_2 (UserInterface|CreateWidget "/Game/Experiment/UI/WBP_ExperimentSetUpPanel.WBP_ExperimentSetUpPanel_C" _returnvalue))
  (UserInterface|Viewport|AddtoViewport _returnvalue_2 0)
  (bind _output_get (Variables|Default|SetExperimentSetUpWidget _returnvalue_2))
  (Variables|/Game/Experiment/UI/WBP_ExperimentSetUpPanel.WBP_ExperimentSetUpPanel_C|SetOwner _output_get self)
  (Default|InitPanel _output_get))

(event Custom|SetLastExperimentData
  (bind _lastexperimentdatatable (Variables|ExperimentData|GetLastExperimentDataTable))
  (bind _returnvalue (Utilities|GetDataTableRow (.datatable _lastexperimentdatatable) (.rowname _lastexperimentdatatable))
    (:then
      (bind _output_get (Variables|ExperimentData|SetLastExperimentData _returnvalue))
      (Variables|ExperimentData|SetNextExperimentData _output_get))))

(event Custom|SetUserIDsData
  (bind _useridsdatatable (Variables|UserIDs|GetUserIDsDataTable))
  (bind _returnvalue (Utilities|GetDataTableRow (.datatable _useridsdatatable) (.rowname _useridsdatatable))
    (:then
      (Variables|UserIDs|SetUserIDsLists (Utilities|Struct|BreakF_ExperimentUserIDs _returnvalue)))))

(event EventBeginPlay
  (CallFunction|SetUserIDsData)
  (CallFunction|SetLastExperimentData)
  (CallFunction|InitExperimentSetUpPanel))

(fn ConstructionScript)

(fn GetUserListbyGroupType
  (params (GroupType :type E_UserGroup%20Enum :default "NewEnumerator0"))
  (for _array_element (Variables|UserIDs|GetUserIDsLists)
    (if (Utilities|Enum|Equal(Enum) (.GroupType (Utilities|Struct|BreakF_UsersIDsByGroupsList _array_element)) GroupType)
      (return (.IDs (Utilities|Struct|BreakF_UsersIDsByGroupsList _array_element)))))
  (return 0))

(fn GetUserIDbyIndex
  (params (GroupType :type E_UserGroup%20Enum :default "NewEnumerator0") (Index :type Integer))
  (return (Utilities|Array|Get(acopy) (CallFunction|GetUserListbyGroupType GroupType) Index)))

(fn GetNextUser
  (params (SelectionType :type E_UserSelectionType%20Enum :default "NewEnumerator0") (Increase :type Integer))
  (Utilities|FlowControl|Sequence
    (:then_0
      (switch Utilities|FlowControl|Switch|SwitchonE_UserSelectionType SelectionType
        (:NewEnumerator0
          (bind (_nextgroup _nextuserindexbygroup) (CallFunction|GetNextAlternateUser (.grouptype (Variables|ExperimentData|GetNextExperimentData)) (.userindexesbygroup (Variables|ExperimentData|GetNextExperimentData)) Increase))
          (LocalVariables|SetNextUserGroup _nextgroup)
          (LocalVariables|SetIndexesUpdated _nextuserindexbygroup))
        (:NewEnumerator1
          (bind (_nextgroup_2 _nextuserindexbygroup_2) (CallFunction|GetNextContinuousUser (.grouptype (Variables|ExperimentData|GetNextExperimentData)) (.userindexesbygroup (Variables|ExperimentData|GetNextExperimentData)) Increase))
          (LocalVariables|SetNextUserGroup _nextgroup_2)
          (LocalVariables|SetIndexesUpdated _nextuserindexbygroup_2))))
    (:then_1
      (Variables|ExperimentData|SetNextExperimentData (Utilities|Struct|MakeF_UserExperimentData SelectionType (CallFunction|GetNextUserID (LocalVariables|GetNextUserGroup) (LocalVariables|GetIndexesUpdated)) (LocalVariables|GetNextUserGroup) "" (LocalVariables|GetIndexesUpdated))))))

(fn ResetNextUser
  (Variables|ExperimentData|SetNextExperimentData (Variables|ExperimentData|GetLastExperimentData)))

(fn GetNextAlternateUser
  (params (CurrentGroup :type E_UserGroup%20Enum :default "NewEnumerator0") (UserIndexByGroup :type Map%20of%20E_UserGroup%20Enums%20to%20Integers :default "NewEnumerator0") (Increase :type Integer))
  (bind _result (Math|Integer|IncrementInt (Math|Conversions|ToInteger(Byte) CurrentGroup))
    (:%20%20
      (Utilities|Map|Add UserIndexByGroup (Utilities|Enum|ByteToEnumE_UserGroup (Math|Conversions|ToByte(Integer) (CallFunction|WrapInteger _result 0 (|GetNumEnumEntries)))) (Math|Integer|Clamp(Integer) (+ (.Value (Utilities|Map|Find UserIndexByGroup (Utilities|Enum|ByteToEnumE_UserGroup (Math|Conversions|ToByte(Integer) (CallFunction|WrapInteger _result 0 (|GetNumEnumEntries)))))) Increase) 0 (- (Utilities|Array|Length (CallFunction|GetListOfIDsbyGroup (Utilities|Enum|ByteToEnumE_UserGroup (Math|Conversions|ToByte(Integer) (CallFunction|WrapInteger _result 0 (|GetNumEnumEntries)))))) 1)))
      (return (Utilities|Enum|ByteToEnumE_UserGroup (Math|Conversions|ToByte(Integer) (CallFunction|WrapInteger _result 0 (|GetNumEnumEntries)))) UserIndexByGroup))))

(fn GetNextContinuousUser
  (params (CurrentGroup :type E_UserGroup%20Enum :default "NewEnumerator0") (UserIndexByGroup :type Map%20of%20E_UserGroup%20Enums%20to%20Integers :default "NewEnumerator0") (Increase :type Integer))
  (Utilities|Map|Add UserIndexByGroup CurrentGroup (Math|Integer|Clamp(Integer) (+ (.Value (Utilities|Map|Find UserIndexByGroup CurrentGroup)) Increase) 0 (- (Utilities|Array|Length (CallFunction|GetListOfIDsbyGroup CurrentGroup)) 1)))
  (return CurrentGroup UserIndexByGroup))

(fn GetNextUserID
  (params (NextUserGroup :type E_UserGroup%20Enum :default "NewEnumerator0") (NextUserIndexByGroup :type Map%20of%20E_UserGroup%20Enums%20to%20Integers :default "NewEnumerator0"))
  (return (Utilities|Array|Get(acopy) (CallFunction|GetListOfIDsbyGroup NextUserGroup) (.Value (Utilities|Map|Find NextUserIndexByGroup NextUserGroup)))))

(fn GetListOfIDsbyGroup
  (params (GroupType :type E_UserGroup%20Enum :default "NewEnumerator0"))
  (for _array_element (Variables|UserIDs|GetUserIDsLists)
    (if (Utilities|Enum|Equal(Enum) (.GroupType (Utilities|Struct|BreakF_UsersIDsByGroupsList _array_element)) GroupType)
      (return (.IDs (Utilities|Struct|BreakF_UsersIDsByGroupsList _array_element)))))
  (return 0))