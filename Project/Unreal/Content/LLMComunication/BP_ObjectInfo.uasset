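; Actor component that describes its owning object as JSON and registers it with the StateManager, as part of the LLM communication system.
; One tick after BeginPlay it finds the StateManager and registers the owner, cast to InteractiveObj, by name.
; CreateObjectInfo serializes name, summary, creator and the owner's LLMInstantiableComponents into a JSON string.
; It also reports whether the object can be grabbed, and DeleteObject unregisters and destroys the owner.
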(event Custom|Register
  (bind _name (Variables|Default|GetName))
  (bind _outactors (Actor|GetAllActorsOfClass "/Game/LLMComunication/StateManager.StateManager_C"))
  (Variables|Default|SetStateManager (Utilities|Array|Get(acopy) _outactors))
  (bind _asinteractive_obj (Utilities|Casting|CastToInteractiveObj (Components|GetOwner self)))
  (Utilities|IsValid (Variables|Default|GetStateManager)
    (:Is%20Valid
      (Default|RegisterObject (Variables|Default|GetStateManager) _asinteractive_obj _name)
      (Default|SetInfo (Variables|Default|GetStateManager) _name))))

(event EventBeginPlay
  (bind _outjsonobject (Class|JsonBlueprintFunctionLibrary|FromString "{}"))
  (bind _output_get (Variables|Default|SetJSON _outjsonobject))
  (Class|KismetSystemLibrary|SetTimerforNextTickDelegate (delegate Custom|Register)))

(fn IsInteractuable
  (return (Variables|Default|GetCanBeGrab)))

(fn DeleteObject
  (Default|UnregisterObject (Variables|Default|GetStateManager) (Variables|Default|GetName))
  (Actor|DestroyActor (Components|GetOwner self)))

(fn SetComponentsField
  (params (json :type Json%20Object%20Wrapper%20Structure))
  (bind _components (LocalVariables|Getcomponents))
  (for _array_element (Actor|GetComponentsByClass (Components|GetOwner) "/Game/LLMComunication/Components/LLMInstantiableComponent.LLMInstantiableComponent_C")
    (bind _serializedjson (Default|GetSerializedComponent _array_element))
    (Utilities|Array|Add _components _serializedjson))
  (|SetJsonField json "components" _components))

(fn CreateObjectInfo
  (bind _json (LocalVariables|Getjson))
  (|SetJsonField _json "name" (Variables|Default|GetName))
  (|SetJsonField _json "summary" (Variables|Default|GetDescription))
  (|SetJsonField _json "creator" (Variables|Default|GetCreator))
  (CallFunction|SetComponentsField _json)
  (bind _outjsonstring (Class|JsonBlueprintFunctionLibrary|ToString _json))
  (return _outjsonstring))